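; BP_Remy is an actor, apparently a character, that turns, moves vertically and shows veins during a collection sequence.
; Each Tick it reads state flags to apply one-shot 90-degree turns or small fixed per-frame up and down offsets, without delta-time scaling.
; While sitting, collecting and closing the hand, it spawns two vein actors once.
; When that state ends, it destroys them through GetAllActorsOfClass lookups.
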(event `self.ReceiveBeginPlay`
  (set `self.goingUp` false)
  (set `self.goingDown` false))

(event `self.ReceiveTick`
  (params (DeltaSeconds :type "Float (single-precision)"))
  (bind _veiasspawned (`self.veiasSpawned`))
  (set `self.finishedTurn` false)
  (`self.RotateRightIfCondition` (`self.rotateRight`))
  (`self.RotateLeftIfCondition` (`self.rotateLeft`))
  (`self.GoUpIfCondition` (`self.goingUp`))
  (`self.goDownIfCondition` (`self.goingDown`))
  (if (and (`self.isSitting`) (`self.isCollecting`) (`self.closeHand`))
    (if (not _veiasspawned)
      (`self.spawnVeias`)
      (set `self.veiasSpawned` true))
    (elif _veiasspawned
      (`self.deleteVeias`)
      (set `self.veiasSpawned` false))))

(fn `deleteVeias`
  (bind _outactors (`GameplayStatics.GetAllActorsOfClass` null))
  (`self.K2_DestroyActor` (`|GetArrayItem` _outactors))
  (bind _outactors_2 (`GameplayStatics.GetAllActorsOfClass` null))
  (`self.K2_DestroyActor` (`|GetArrayItem` _outactors_2)))

(fn `goDownIfCondition`
  (params (Condition :type Boolean))
  (if Condition
    (`self.K2_AddActorWorldOffset` (0.0 0.0 -0.3))
    (return)
    (else
      (return))))

(fn `GoUpIfCondition`
  (params (Condition :type Boolean))
  (if Condition
    (`self.K2_AddActorWorldOffset` (-0.1 0.0 0.4))
    (return)
    (else
      (return))))

(fn `RotateLeftIfCondition`
  (params (Condition :type Boolean))
  (if Condition
    (set `self.rotateLeft` false)
    (set `self.turnLeft` false)
    (`self.K2_AddActorWorldRotation` (struct :`Yaw` -90.0))
    (return)
    (else
      (return))))

(fn `RotateRightIfCondition`
  (params (Condition :type Boolean))
  (if Condition
    (set `self.rotateRight` false)
    (set `self.turnRight` false)
    (`self.K2_AddActorWorldRotation` (struct :`Yaw` 90.0))
    (set `self.finishedTurn` true)
    (return)
    (else
      (return))))

(fn `spawnVeias`
  (`|SpawnActorFromClass` (`self.BP_Vein 1`) (`self.veia1Transform`) "Undefined" "MultiplyWithRoot" null null)
  (`|SpawnActorFromClass` (`self.BP_Vein 2`) (`self.veia2Transform`) "Undefined" "MultiplyWithRoot" null null))

(fn `UserConstructionScript`)