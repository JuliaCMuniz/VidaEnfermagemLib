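; Demo patient for a VR nursing blood-collection exercise, with decals for arm veins and asepsis.
; BeginPlay creates dynamic materials for both decals.
; Tick, gated on ReferenciasSetadas, derives fist and collection animation flags from player proximity and syringe state, then updates vein opacity.
; SetarReferencias is empty and its lookup loop is disconnected, so nothing here sets that gate; the vein fade-out function is never called.
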(event `self.ReceiveBeginPlay`
  (`self.setup`))

(event `self.ReceiveTick`
  (params (DeltaSeconds :type "Float (single-precision)"))
  (if (`self.ReferenciasSetadas`)
    (`self.DefineAnimação`)
    (`self.DefineOpacidadeDecal`)
    (`self.MostrarVeias`)))

(fn `DefineAnimação`
  (locals (`ComeçouColeta` :type Boolean :default false) (PosicaoJogador :type "Vector Structure"))
  (bind _outactors (`GameplayStatics.GetAllActorsOfClass` "/Game/VIDAEnfermagem/Characters/Player/BP_FloatingHands.BP_FloatingHands_C"))
  (if (`HeadMountedDisplayFunctionLibrary.IsHeadMountedDisplayEnabled`)
    (bind _output (`|GetArrayItem` _outactors))
    (set `local.PosicaoJogador` (`SceneComponent.K2_GetComponentLocation` (`/Game/VIDAEnfermagem/Characters/Player/BP_FloatingHands.Camera` _output)))
    (else
      (set `local.PosicaoJogador` (`self.K2_GetActorLocation` _output))))
  (bind _outactors_2 (`GameplayStatics.GetAllActorsOfClass` "/Game/VIDAEnfermagem/Pickables/Syringe/BP_Syringe.BP_Syringe_C"))
  (bind _output_2 (`|GetArrayItem` _outactors_2))
  (set `local.ComeçouColeta` (or (`/Game/VIDAEnfermagem/Pickables/Syringe/BP_Syringe.naVeia` _output_2) (`/Game/VIDAEnfermagem/Pickables/Syringe/BP_Syringe.noBraço` _output_2)))
  (set `self.MaoFechada` (or (== _output_2 (`/Game/VIDAEnfermagem/Characters/Player/BP_FloatingHands.ObjetoAnexadoDireita` _output)) (== _output_2 (`/Game/VIDAEnfermagem/Characters/Player/BP_FloatingHands.ObjetoAnexadoEsquerda` _output)) (`local.ComeçouColeta`)))
  (set `self.Coletando` (or (`local.ComeçouColeta`) (<= (`self.CalculaDistancia` (`local.PosicaoJogador`) (`self.K2_GetActorLocation`)) 90.0)))
  (return))

(fn `DefineOpacidadeDecal`
  (locals (Max :type "Float (double-precision)") (Min :type "Float (double-precision)"))
  (bind _output_get (set `local.Max` 0.9))
  (bind _output_get_2 (set `self.VeiasMaxDecalOpacity` _output_get))
  (set `self.VeiasMinDecalOpacity` _output_get_2)
  (return))

(fn `EsconderVeias`
  (bind _veiasopacity (`self.VeiasOpacity`))
  (if (<= _veiasopacity (`self.VeiasMinDecalOpacity`))
    (set `self.FadeOutVeias` false)
    (else
      (bind _output_get (set `self.VeiasOpacity` (- _veiasopacity (`self.VeiasFadeSpeed`))))
      (`MaterialInstanceDynamic.SetScalarParameterValue` (`self.DecalMaterial`) "Opacity" _output_get)))
  (return))

(fn `MostrarVeias`
  (`MaterialInstanceDynamic.SetScalarParameterValue` (`self.DecalMaterial`) "Opacity" (`self.VeiasOpacity`))
  (return))

(fn `SetarReferencias`)

(fn `setup`
  (bind _decalassepsia (`self.DecalAssepsia`))
  (bind _decalveia (`self.DecalVeia`))
  (`self.SetarReferencias`)
  (bind _returnvalue (`KismetMaterialLibrary.CreateDynamicMaterialInstance` (`DecalComponent.GetDecalMaterial` _decalveia) "/Game/VIDAEnfermagem/MaterialLibrary/M_Veia.M_Veia"))
  (bind _output_get (set `self.DecalMaterial` _returnvalue))
  (`DecalComponent.SetDecalMaterial` _decalveia _output_get)
  (bind _returnvalue_2 (`KismetMaterialLibrary.CreateDynamicMaterialInstance` (`DecalComponent.GetDecalMaterial` _decalassepsia) "/Game/VIDAEnfermagem/MaterialLibrary/Assepsia/M_Asepsis.M_Asepsis"))
  (bind _output_get_2 (set `self.AssepsiaDecalMaterial` _returnvalue_2))
  (`DecalComponent.SetDecalMaterial` _decalassepsia _output_get_2)
  (cast `/Game/VIDAEnfermagem/Core/LeapGameMode` (`GameplayStatics.GetGameMode`)))

(fn `UserConstructionScript`)