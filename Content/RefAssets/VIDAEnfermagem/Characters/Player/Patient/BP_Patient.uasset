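; Patient actor for a Leap Motion nursing blood-collection simulation, reacting to tourniquet, asepsis, skin-pull and dry-cotton steps.
; Pinches attach or remove the tourniquet; tourniquet and asepsis steps are written to a report.
; Trigger overlaps detect wet cotton for asepsis and swap player hands for posed pull or cotton meshes.
; Tick sets animation flags and fades dynamic-material decals, with vein opacity limits driven by tourniquet and pull state.
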(event `Key|LeapPinchR` :consume false
  (params (Key :type "Key Structure"))
  (:`Pressed`
    (`self.SoltarGarroteDoBraço` :!label _label)
    (`KismetSystemLibrary.K2_ClearTimer` null "PrenderGarroteNoBraço"))
  (:`Released`
    (if (not (`self.Garroteado`))
      (`KismetSystemLibrary.K2_SetTimer` null "PrenderGarroteNoBraço" 0.2 :!label _label_2))))

(event `Key|LeapPinchL` :consume false
  (params (Key :type "Key Structure"))
  (:`Pressed`
    (goto _label))
  (:`Released`
    (if (not (`self.Garroteado`))
      (goto _label_2))))

(event `self.TriggerAssepsia.OnComponentBeginOverlap`
  (params (OverlappedComponent :type "PrimitiveComponent Object Reference") (OtherActor :type "Actor Object Reference") (OtherComp :type "PrimitiveComponent Object Reference") (OtherBodyIndex :type Integer) (bFromSweep :type Boolean) (SweepResult :type "HitResult Structure (by ref)"))
  (cast `/Game/VIDAEnfermagem/Pickables/Cotton/BP_Cotton_Wet` OtherActor)
  (if (not (`self.AssepsiaRealizada`))
    (set `self.AssepsiaRealizada` true)
    (`/Game/VIDAEnfermagem/Core/WriteText.EscreveRelatorio` "Realizou Asspesia")
    (set `self.FadeInAssepsia` true)
    (`KismetSystemLibrary.Delay` 4.0)
    (set `self.FadeOutAssepsia` true)))

(event `self.ReceiveBeginPlay`
  (`self.setup`))

(event `self.ReceiveTick`
  (params (DeltaSeconds :type "Float (single-precision)"))
  (if (`self.ReferenciasSetadas`)
    (`self.DefineAnimação`)
    (`self.DefineOpacidadeDecal`)
    (if (`self.FadeInVeias`)
      (`self.MostrarVeias`)
      (elif (`self.FadeOutVeias`)
        (`self.EsconderVeias`)))
    (if (`self.FadeInAssepsia`)
      (`self.MostrarAssepsia`)
      (elif (`self.FadeOutAssepsia`)
        (`self.EsconderAssepsia`)))))

(event `self.TriggerPuxada.OnComponentBeginOverlap`
  (params (OverlappedComponent :type "PrimitiveComponent Object Reference") (OtherActor :type "Actor Object Reference") (OtherComp :type "PrimitiveComponent Object Reference") (OtherBodyIndex :type Integer) (bFromSweep :type Boolean) (SweepResult :type "HitResult Structure (by ref)"))
  (bind _returnvalue (`KismetSystemLibrary.GetObjectName` OtherComp))
  (bind `_intermediário_referência` (`self.Intermediário Referência`))
  (bind _returnvalue_2 (not (`/Game/VIDAEnfermagem/Pickables/Syringe/BP_Syringe.noBraço` `_intermediário_referência`)))
  (bind _returnvalue_3 (not (`/Game/VIDAEnfermagem/Pickables/Syringe/BP_Syringe.ProcedimentoEmProgresso` `_intermediário_referência`)))
  (if (`self.ReferenciasSetadas`)
    (if (and (`KismetStringLibrary.EqualEqual_StrStr` _returnvalue "Left") (== (`/Game/VIDAEnfermagem/Characters/Player/BP_FloatingHands.ObjetoAnexadoEsquerda` (`self.JogadorReferencia`)) null) _returnvalue_3 _returnvalue_2)
      (`self.MostraMãoEsquerdaPuxada`)
      (elif (and (`KismetStringLibrary.EqualEqual_StrStr` _returnvalue "Right") _returnvalue_3 _returnvalue_2 (== (`/Game/VIDAEnfermagem/Characters/Player/BP_FloatingHands.ObjetoAnexadoDireita` (`self.JogadorReferencia`)) null))
        (`self.MostraMãoDireitaPuxada`)))))

(event `self.TriggerPuxada.OnComponentEndOverlap`
  (params (OverlappedComponent :type "PrimitiveComponent Object Reference") (OtherActor :type "Actor Object Reference") (OtherComp :type "PrimitiveComponent Object Reference") (OtherBodyIndex :type Integer))
  (if (and (`KismetStringLibrary.EqualEqual_StrStr` (`KismetSystemLibrary.GetObjectName` OtherComp) "Left") (`SceneComponent.IsVisible` (`self.MaoEsquerdaPuxada`)))
    (`self.EscondeMãoEsquerdaPuxada`)
    (elif (and (`KismetStringLibrary.EqualEqual_StrStr` (`KismetSystemLibrary.GetObjectName` OtherComp) "Right") (`SceneComponent.IsVisible` (`self.MaoDireitaPuxada`)))
      (`self.EscondeMãoDireitaPuxada`))))

(event `self.TriggerAlgodão.OnComponentBeginOverlap`
  (params (OverlappedComponent :type "PrimitiveComponent Object Reference") (OtherActor :type "Actor Object Reference") (OtherComp :type "PrimitiveComponent Object Reference") (OtherBodyIndex :type Integer) (bFromSweep :type Boolean) (SweepResult :type "HitResult Structure (by ref)"))
  (bind _coletorreferencia (`self.ColetorReferencia`))
  (if (`KismetSystemLibrary.IsValid` _coletorreferencia)
    (if (and (`KismetStringLibrary.EqualEqual_StrStr` (`KismetSystemLibrary.GetObjectName` OtherComp) "AlgodãoSeco") (`/Game/VIDAEnfermagem/Pickables/CollectionTube/BP_CollectionTube.bProcedureInProgress` _coletorreferencia) (not (`/Game/VIDAEnfermagem/Pickables/CollectionTube/BP_CollectionTube.bAttachedToSyringe` _coletorreferencia)))
      (`self.MostraMãoAlgodão`)
      (set `/Game/VIDAEnfermagem/Pickables/CollectionTube/BP_CollectionTube.bProcedureInProgress` false _coletorreferencia))))

(event `self.TriggerAlgodão.OnComponentEndOverlap`
  (params (OverlappedComponent :type "PrimitiveComponent Object Reference") (OtherActor :type "Actor Object Reference") (OtherComp :type "PrimitiveComponent Object Reference") (OtherBodyIndex :type Integer))
  (if (`KismetStringLibrary.EqualEqual_StrStr` (`KismetSystemLibrary.GetObjectName` OtherComp) "AlgodãoSeco")
    (`self.EscondeMãoAlgodão`)))

(fn `DefineAnimação`
  (locals (`ComeçouColeta` :type Boolean :default false) (PosicaoJogador :type "Vector Structure"))
  (bind _outactors (`GameplayStatics.GetAllActorsOfClass` "/Game/VIDAEnfermagem/Characters/Player/BP_FloatingHands.BP_FloatingHands_C"))
  (if (`HeadMountedDisplayFunctionLibrary.IsHeadMountedDisplayEnabled`)
    (bind _output (`|GetArrayItem` _outactors))
    (set `local.PosicaoJogador` (`SceneComponent.K2_GetComponentLocation` (`/Game/VIDAEnfermagem/Characters/Player/BP_FloatingHands.Camera` _output)))
    (else
      (set `local.PosicaoJogador` (`self.K2_GetActorLocation` _output))))
  (bind _outactors_2 (`GameplayStatics.GetAllActorsOfClass` "/Game/VIDAEnfermagem/Pickables/Syringe/BP_Syringe.BP_Syringe_C"))
  (bind _output_2 (`|GetArrayItem` _outactors_2))
  (set `local.ComeçouColeta` (or (`/Game/VIDAEnfermagem/Pickables/Syringe/BP_Syringe.naVeia` _output_2) (`/Game/VIDAEnfermagem/Pickables/Syringe/BP_Syringe.noBraço` _output_2) (`self.Garroteado`)))
  (set `self.MaoFechada` (or (== _output_2 (`/Game/VIDAEnfermagem/Characters/Player/BP_FloatingHands.ObjetoAnexadoDireita` _output)) (== _output_2 (`/Game/VIDAEnfermagem/Characters/Player/BP_FloatingHands.ObjetoAnexadoEsquerda` _output)) (`local.ComeçouColeta`) (`self.Puxada`)))
  (set `self.Coletando` (or (`local.ComeçouColeta`) (<= (`self.CalculaDistancia` (`local.PosicaoJogador`) (`self.K2_GetActorLocation`)) 90.0)))
  (return))

(fn `DefineOpacidadeDecal`
  (locals (Max :type "Float (double-precision)") (Min :type "Float (double-precision)"))
  (bind _output_get (set `local.Max` 0.0))
  (if (`self.Puxada`)
    (bind _output_get_2 (set `local.Max` (+ _output_get 0.4))))
  (if (`self.Garroteado`)
    (bind _output_get_3 (set `local.Max` (+ _output_get_2 0.5))))
  (set `self.VeiasMaxDecalOpacity` _output_get_3)
  (bind _output_get_4 (set `local.Min` 0.9))
  (if (not (`self.Puxada`))
    (bind _output_get_5 (set `local.Min` (- _output_get_4 0.4))))
  (if (not (`self.Garroteado`))
    (bind _output_get_6 (set `local.Min` (- _output_get_5 0.5))))
  (set `self.VeiasMinDecalOpacity` _output_get_6)
  (return))

(fn `EscondeMãoAlgodão`
  (`SceneComponent.SetVisibility` (`self.AlgodaoSeco`) false false)
  (if (`SceneComponent.IsVisible` (`self.MaoEsquerdaAlgodaoSeco`))
    (`SceneComponent.SetVisibility` (`self.MaoEsquerdaAlgodaoSeco`) false false)
    (bind (_right _left) (`/Game/VIDAEnfermagem/Characters/Player/BP_FloatingHands.GetHandMeshes` (`self.JogadorReferencia`)))
    (`SceneComponent.SetVisibility` _left true true)
    (`self.SetarReferencias`)
    (else
      (`SceneComponent.SetVisibility` (`self.MaoDireitaAlgodaoSeco`) false false)
      (bind _right_2 (`/Game/VIDAEnfermagem/Characters/Player/BP_FloatingHands.GetHandMeshes` (`self.JogadorReferencia`)))
      (`SceneComponent.SetVisibility` _right_2 true true)
      (`self.SetarReferencias`))))

(fn `EscondeMãoDireitaPuxada`
  (if (`self.Puxada`)
    (set `self.FadeOutVeias` true)
    (bind _right (`/Game/VIDAEnfermagem/Characters/Player/BP_FloatingHands.GetHandMeshes` (`self.JogadorReferencia`)))
    (`SceneComponent.SetVisibility` _right true false)
    (`SceneComponent.SetVisibility` (`self.MaoDireitaPuxada`) false false)
    (set `self.Puxada` false)))

(fn `EscondeMãoEsquerdaPuxada`
  (if (`self.Puxada`)
    (set `self.FadeOutVeias` true)
    (bind (_right _left) (`/Game/VIDAEnfermagem/Characters/Player/BP_FloatingHands.GetHandMeshes` (`self.JogadorReferencia`)))
    (`SceneComponent.SetVisibility` _left true false)
    (`SceneComponent.SetVisibility` (`self.MaoEsquerdaPuxada`) false false)
    (set `self.Puxada` false)))

(fn `EsconderAssepsia`
  (bind _assepsiaopacity (`self.AssepsiaOpacity`))
  (if (<= _assepsiaopacity (`self.AssepsiaMinDecalOpacity`))
    (set `self.FadeOutAssepsia` false)
    (else
      (bind _output_get (set `self.AssepsiaOpacity` (- _assepsiaopacity (`self.AssepsiaFadeSpeed`))))
      (`MaterialInstanceDynamic.SetScalarParameterValue` (`self.AssepsiaDecalMaterial`) "Opacity" _output_get)))
  (return))

(fn `EsconderVeias`
  (bind _veiasopacity (`self.VeiasOpacity`))
  (if (<= _veiasopacity (`self.VeiasMinDecalOpacity`))
    (set `self.FadeOutVeias` false)
    (else
      (bind _output_get (set `self.VeiasOpacity` (- _veiasopacity (`self.VeiasFadeSpeed`))))
      (`MaterialInstanceDynamic.SetScalarParameterValue` (`self.DecalMaterial`) "Opacity" _output_get)))
  (return))

(fn `MostraMãoAlgodão`
  (bind `_intermediário_referência` (`self.Intermediário Referência`))
  (bind _jogadorreferencia (`self.JogadorReferencia`))
  (`SceneComponent.SetVisibility` (`self.AlgodaoSeco`) true false)
  (`SceneComponent.K2_SetWorldLocation` (`self.AlgodaoSeco`) (+ (`SceneComponent.K2_GetComponentLocation` (`/Game/VIDAEnfermagem/Pickables/Syringe/BP_Syringe.Meia Ponta` (`self.Intermediário Referência`))) (0.0 0.0 2.0)) false false)
  (set `/Game/VIDAEnfermagem/Pickables/Syringe/BP_Syringe.ProcedimentoEmProgresso` false (`self.Intermediário Referência`))
  (`/Game/VIDAEnfermagem/Pickables/Syringe/BP_Syringe.EsconderMãoFantasma` (`self.Intermediário Referência`))
  (if (`/Game/VIDAEnfermagem/Pickables/Syringe/BP_Syringe.ProcedimentoMaoDireita` `_intermediário_referência`)
    (`SceneComponent.SetVisibility` (`self.MaoEsquerdaAlgodaoSeco`) true false)
    (bind (_right _left) (`/Game/VIDAEnfermagem/Characters/Player/BP_FloatingHands.GetHandMeshes` _jogadorreferencia))
    (`SceneComponent.SetVisibility` _left false true)
    (elif (`/Game/VIDAEnfermagem/Pickables/Syringe/BP_Syringe.ProcedimentoMaoEsquerda` `_intermediário_referência`)
      (`SceneComponent.SetVisibility` (`self.MaoDireitaAlgodaoSeco`) true false)
      (bind _right_2 (`/Game/VIDAEnfermagem/Characters/Player/BP_FloatingHands.GetHandMeshes` _jogadorreferencia))
      (`SceneComponent.SetVisibility` _right_2 false true))))

(fn `MostraMãoDireitaPuxada`
  (set `self.FadeInVeias` true)
  (bind _right (`/Game/VIDAEnfermagem/Characters/Player/BP_FloatingHands.GetHandMeshes` (`self.JogadorReferencia`)))
  (`SceneComponent.SetVisibility` _right false false)
  (`SceneComponent.SetVisibility` (`self.MaoDireitaPuxada`) true false)
  (set `self.Puxada` true))

(fn `MostraMãoEsquerdaPuxada`
  (set `self.FadeInVeias` true)
  (bind (_right _left) (`/Game/VIDAEnfermagem/Characters/Player/BP_FloatingHands.GetHandMeshes` (`self.JogadorReferencia`)))
  (`SceneComponent.SetVisibility` _left false false)
  (`SceneComponent.SetVisibility` (`self.MaoEsquerdaPuxada`) true false)
  (set `self.Puxada` true))

(fn `MostrarAssepsia`
  (bind _assepsiaopacity (`self.AssepsiaOpacity`))
  (if (>= _assepsiaopacity (`self.AssepsiaMaxDecalOpacity`))
    (set `self.FadeInAssepsia` false)
    (else
      (bind _output_get (set `self.AssepsiaOpacity` (+ _assepsiaopacity (`self.AssepsiaFadeSpeed`))))
      (`MaterialInstanceDynamic.SetScalarParameterValue` (`self.AssepsiaDecalMaterial`) "Opacity" _output_get)))
  (return))

(fn `MostrarVeias`
  (bind _veiasopacity (`self.VeiasOpacity`))
  (if (>= _veiasopacity (`self.VeiasMaxDecalOpacity`))
    (set `self.FadeInVeias` false)
    (else
      (bind _output_get (set `self.VeiasOpacity` (+ _veiasopacity (`self.VeiasFadeSpeed`))))
      (`MaterialInstanceDynamic.SetScalarParameterValue` (`self.DecalMaterial`) "Opacity" _output_get)))
  (return))

(fn `PrenderGarroteNoBraço`
  (bind _asbp_floating_hands (cast `/Game/VIDAEnfermagem/Characters/Player/BP_FloatingHands` (`GameplayStatics.GetPlayerCharacter` 0)))
  (bind (_success _tourniquet) (`self.SoltarGarroteDaMão` _asbp_floating_hands))
  (if _success
    (bind _rootcomponent (`Actor.RootComponent` _tourniquet))
    (`SceneComponent.SetVisibility` _rootcomponent true false)
    (set `self.GarroteReferência` _tourniquet)
    (`SceneComponent.K2_SetWorldLocation` _rootcomponent (0.0 0.0 -20.0) false false)
    (`SceneComponent.SetVisibility` (`self.GarrotePreso`) true false)
    (set `self.Garroteado` true)
    (set `self.FadeInVeias` true)
    (`/Game/VIDAEnfermagem/Core/WriteText.EscreveRelatorio` "Garroteou")))

(fn `SetarReferencias`
  (bind _returnvalue (`KismetSystemLibrary.IsValid` (`self.JogadorReferencia`)))
  (bind _returnvalue_2 (`KismetSystemLibrary.IsValid` (`self.GarroteReferência`)))
  (bind _returnvalue_3 (`KismetSystemLibrary.IsValid` (`self.Intermediário Referência`)))
  (bind _returnvalue_4 (`KismetSystemLibrary.IsValid` (`self.ColetorReferencia`)))
  (while (not (`self.ReferenciasSetadas`))
    (if (not _returnvalue)
      (bind _outactors (`GameplayStatics.GetAllActorsOfClass` "/Game/VIDAEnfermagem/Characters/Player/BP_FloatingHands.BP_FloatingHands_C"))
      (set `self.JogadorReferencia` (`|GetArrayItem` _outactors)))
    (if (not _returnvalue_2)
      (bind _outactors_2 (`GameplayStatics.GetAllActorsOfClass` "/Game/VIDAEnfermagem/Pickables/TourniquetBuckle/BP_TourniquetBuckle.BP_TourniquetBuckle_C"))
      (set `self.GarroteReferência` (`|GetArrayItem` _outactors_2)))
    (if _returnvalue_3
      (if (not _returnvalue_4)
        (bind _outactors_3 (`GameplayStatics.GetAllActorsOfClass` "/Game/VIDAEnfermagem/Pickables/CollectionTube/BP_CollectionTube.BP_CollectionTube_C" :!label _label))
        (set `self.ColetorReferencia` (`|GetArrayItem` _outactors_3)))
      (else
        (bind _outactors_4 (`GameplayStatics.GetAllActorsOfClass` "/Game/VIDAEnfermagem/Pickables/Syringe/BP_Syringe.BP_Syringe_C"))
        (set `self.Intermediário Referência` (`|GetArrayItem` _outactors_4))
        (goto _label)))
    (set `self.ReferenciasSetadas` (and _returnvalue _returnvalue_2 _returnvalue_3 _returnvalue_4))))

(fn `setup`
  (bind _decalassepsia (`self.DecalAssepsia`))
  (bind _decalveia (`self.DecalVeia`))
  (`self.SetarReferencias`)
  (`SceneComponent.SetVisibility` (`self.GarrotePreso`) false false)
  (set `self.Garroteado` false)
  (bind _returnvalue (`KismetMaterialLibrary.CreateDynamicMaterialInstance` (`DecalComponent.GetDecalMaterial` _decalveia) "/Game/VIDAEnfermagem/MaterialLibrary/M_Veia.M_Veia"))
  (bind _output_get (set `self.DecalMaterial` _returnvalue))
  (`DecalComponent.SetDecalMaterial` _decalveia _output_get)
  (bind _returnvalue_2 (`KismetMaterialLibrary.CreateDynamicMaterialInstance` (`DecalComponent.GetDecalMaterial` _decalassepsia) "/Game/VIDAEnfermagem/MaterialLibrary/Assepsia/M_Asepsis.M_Asepsis"))
  (bind _output_get_2 (set `self.AssepsiaDecalMaterial` _returnvalue_2))
  (`DecalComponent.SetDecalMaterial` _decalassepsia _output_get_2)
  (cast `/Game/VIDAEnfermagem/Core/LeapGameMode` (`GameplayStatics.GetGameMode`)))

(fn `SoltarGarroteDaMão`
  (params (In :type "/Game/VIDAEnfermagem/Characters/Player/BP_FloatingHands Object Reference"))
  (returns (Success :type Boolean) (Tourniquet :type "/Game/VIDAEnfermagem/Pickables/TourniquetBuckle/BP_TourniquetBuckle Object Reference"))
  (if (`/Game/VIDAEnfermagem/Characters/Player/BP_FloatingHands.PegandoDireita` In)
    (bind _asbp_tourniquet_buckle (cast `/Game/VIDAEnfermagem/Pickables/TourniquetBuckle/BP_TourniquetBuckle` (`/Game/VIDAEnfermagem/Characters/Player/BP_FloatingHands.ObjetoAnexadoDireita` In))
      (:`then`
        (if (`/Game/VIDAEnfermagem/Pickables/TourniquetBuckle/BP_TourniquetBuckle.bOverlappingPatient` _asbp_tourniquet_buckle)
          (`/Game/VIDAEnfermagem/Characters/Player/BP_FloatingHands.Soltar_D` In)
          (return true _asbp_tourniquet_buckle)
          (else
            (return false null))))
      (:`CastFailed`
        _)))
  (if (`/Game/VIDAEnfermagem/Characters/Player/BP_FloatingHands.PegandoEsquerda` In)
    (bind _asbp_tourniquet_buckle_2 (cast `/Game/VIDAEnfermagem/Pickables/TourniquetBuckle/BP_TourniquetBuckle` (`/Game/VIDAEnfermagem/Characters/Player/BP_FloatingHands.ObjetoAnexadoEsquerda` In)))
    (if (`/Game/VIDAEnfermagem/Pickables/TourniquetBuckle/BP_TourniquetBuckle.bOverlappingPatient` _asbp_tourniquet_buckle_2)
      (`/Game/VIDAEnfermagem/Characters/Player/BP_FloatingHands.Soltar_E` In)
      (return true _asbp_tourniquet_buckle_2)
      (else
        (return false null)))))

(fn `SoltarGarroteDoBraço`
  (bind _jogadorreferencia (`self.JogadorReferencia`))
  (bind `_garrotereferência` (`self.GarroteReferência`))
  (bind _garrotepreso (`self.GarrotePreso`))
  (bind _asbp_floating_hands (cast `/Game/VIDAEnfermagem/Characters/Player/BP_FloatingHands` (`GameplayStatics.GetPlayerCharacter` 0)))
  (if (`self.Garroteado`)
    (bind _asbp_custom_leap_low_poly_hand (cast `/Game/VIDAEnfermagem/Core/Leap/BP_CustomLeapLowPolyHand` (`ChildActorComponent.ChildActor` (`/Game/VIDAEnfermagem/Characters/Player/BP_FloatingHands.LeapHands` _asbp_floating_hands))))
    (if (and (not (`/Game/VIDAEnfermagem/Characters/Player/BP_FloatingHands.PegandoDireita` _asbp_floating_hands)) (`PrimitiveComponent.IsOverlappingComponent` (`/Game/VIDAEnfermagem/Core/Leap/BP_CustomLeapLowPolyHand.Right` _asbp_custom_leap_low_poly_hand) _garrotepreso))
      (set `/Game/VIDAEnfermagem/Characters/Player/BP_FloatingHands.TocandoDireita` true _jogadorreferencia)
      (set `/Game/VIDAEnfermagem/Characters/Player/BP_FloatingHands.ObjetoTocandoDireita` `_garrotereferência` _jogadorreferencia)
      (`SceneComponent.SetVisibility` (`self.GarrotePreso`) false false :!label _label)
      (set `self.Garroteado` false)
      (set `self.FadeOutVeias` true)
      (`/Game/VIDAEnfermagem/Core/WriteText.EscreveRelatorio` "Desgarroteou")
      (elif (and (`PrimitiveComponent.IsOverlappingComponent` (`/Game/VIDAEnfermagem/Core/Leap/BP_CustomLeapLowPolyHand.Left` _asbp_custom_leap_low_poly_hand) _garrotepreso) (not (`/Game/VIDAEnfermagem/Characters/Player/BP_FloatingHands.PegandoEsquerda` _asbp_floating_hands)))
        (set `/Game/VIDAEnfermagem/Characters/Player/BP_FloatingHands.TocandoEsquerda` true _jogadorreferencia)
        (set `/Game/VIDAEnfermagem/Characters/Player/BP_FloatingHands.ObjetoTocandoEsquerda` `_garrotereferência` _jogadorreferencia)
        (goto _label)))))

(fn `UserConstructionScript`)