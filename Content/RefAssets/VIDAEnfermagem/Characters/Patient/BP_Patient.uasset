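; Patient actor for a VR nursing blood-collection exercise, reacting to tourniquet, antisepsis, skin-pull and cotton steps.
; Leap pinches attach or remove the tourniquet, while trigger overlaps handle the other steps, swapping player hands for posed meshes.
; Tourniquet and antisepsis steps write to the report and notify the FSM.
; Tick sets animation flags and fades vein and antisepsis decals through dynamic materials, with tourniquet and pull states setting vein opacity limits.
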(event `InputAxisKey|OculusHand_Right_IndexPinchStrength`
  (params (AxisValue :type "Float (single-precision)")))

(event `Key|LeapPinchR` :consume false
  (params (Key :type "Key Structure"))
  (:`Pressed`
    (`self.SoltarGarroteDoBraço` :!label _label)
    (`KismetSystemLibrary.K2_ClearTimer` null "PrenderGarroteNoBraço"))
  (:`Released`
    (if (not (`self.Garroteado`))
      (`KismetSystemLibrary.K2_SetTimer` null "PrenderGarroteNoBraço" 0.2 :!label _label_2))))

(event `Key|LeapPinchL` :consume false
  (params (Key :type "Key Structure"))
  (:`Pressed`
    (goto _label))
  (:`Released`
    (if (not (`self.Garroteado`))
      (goto _label_2))))

(event `self.TriggerAssepsia.OnComponentBeginOverlap`
  (params (OverlappedComponent :type "PrimitiveComponent Object Reference") (OtherActor :type "Actor Object Reference") (OtherComp :type "PrimitiveComponent Object Reference") (OtherBodyIndex :type Integer) (bFromSweep :type Boolean) (SweepResult :type "HitResult Structure (by ref)"))
  (cast `` OtherActor)
  (if (not (`self.AssepsiaRealizada`))
    (set `self.AssepsiaRealizada` true)
    (`self.EscreveRelatorio` "Realizou Asspesia")
    (set `self.FadeInAssepsia` true)
    (`KismetSystemLibrary.Delay` 4.0)
    (set `self.FadeOutAssepsia` true)
    (`self.PatientSterilyzed` (`.FSM` (`self.FSM`)))))

(event `self.ReceiveBeginPlay`
  (`self.setup`))

(event `self.ReceiveTick`
  (params (DeltaSeconds :type "Float (single-precision)"))
  (if (`self.ReferenciasSetadas`)
    (`self.DefineAnimação`)
    (`self.DefineOpacidadeDecal`)
    (if (`self.FadeInVeias`)
      (`self.MostrarVeias`)
      (elif (`self.FadeOutVeias`)
        (`self.EsconderVeias`)))
    (if (`self.FadeInAssepsia`)
      (`self.MostrarAssepsia`)
      (elif (`self.FadeOutAssepsia`)
        (`self.EsconderAssepsia`)))))

(event `self.TriggerPuxada.OnComponentBeginOverlap`
  (params (OverlappedComponent :type "PrimitiveComponent Object Reference") (OtherActor :type "Actor Object Reference") (OtherComp :type "PrimitiveComponent Object Reference") (OtherBodyIndex :type Integer) (bFromSweep :type Boolean) (SweepResult :type "HitResult Structure (by ref)"))
  (bind _returnvalue (`KismetSystemLibrary.GetObjectName` OtherComp))
  (bind (`_intermediário_referência` `_intermediário_referência_2`) (`self.Intermediário Referência`))
  (bind _returnvalue_2 (not (`/Game/RefAssets/VIDAEnfermagem/Characters/Patient/BP_Patient.noBraço` `_intermediário_referência_2`)))
  (bind _returnvalue_3 (not (`/Game/RefAssets/VIDAEnfermagem/Characters/Patient/BP_Patient.ProcedimentoEmProgresso` `_intermediário_referência_2`)))
  (if (`self.ReferenciasSetadas`)
    (if (and (`KismetStringLibrary.EqualEqual_StrStr` _returnvalue "Left") (== (`/Game/RefAssets/VIDAEnfermagem/Characters/Patient/BP_Patient.ObjetoAnexadoEsquerda` (`.JogadorReferencia` (`self.JogadorReferencia`))) null) _returnvalue_3 _returnvalue_2)
      (`self.MostraMãoEsquerdaPuxada`)
      (elif (and (`KismetStringLibrary.EqualEqual_StrStr` _returnvalue "Right") _returnvalue_3 _returnvalue_2 (== (`/Game/RefAssets/VIDAEnfermagem/Characters/Patient/BP_Patient.ObjetoAnexadoDireita` (`.JogadorReferencia` (`self.JogadorReferencia`))) null))
        (`self.MostraMãoDireitaPuxada`)))))

(event `self.TriggerPuxada.OnComponentEndOverlap`
  (params (OverlappedComponent :type "PrimitiveComponent Object Reference") (OtherActor :type "Actor Object Reference") (OtherComp :type "PrimitiveComponent Object Reference") (OtherBodyIndex :type Integer))
  (if (and (`KismetStringLibrary.EqualEqual_StrStr` (`KismetSystemLibrary.GetObjectName` OtherComp) "Left") (`SceneComponent.IsVisible` (`self.MaoEsquerdaPuxada`)))
    (`self.EscondeMãoEsquerdaPuxada`)
    (elif (and (`KismetStringLibrary.EqualEqual_StrStr` (`KismetSystemLibrary.GetObjectName` OtherComp) "Right") (`SceneComponent.IsVisible` (`self.MaoDireitaPuxada`)))
      (`self.EscondeMãoDireitaPuxada`))))

(event `self.TriggerAlgodão.OnComponentBeginOverlap`
  (params (OverlappedComponent :type "PrimitiveComponent Object Reference") (OtherActor :type "Actor Object Reference") (OtherComp :type "PrimitiveComponent Object Reference") (OtherBodyIndex :type Integer) (bFromSweep :type Boolean) (SweepResult :type "HitResult Structure (by ref)"))
  (bind (_coletorreferencia _coletorreferencia_2) (`self.ColetorReferencia`))
  (if (`KismetSystemLibrary.IsValid` _coletorreferencia_2)
    (if (and (`KismetStringLibrary.EqualEqual_StrStr` (`KismetSystemLibrary.GetObjectName` OtherComp) "AlgodãoSeco") (`/Game/RefAssets/VIDAEnfermagem/Characters/Patient/BP_Patient.bProcedureInProgress` _coletorreferencia_2) (not (`/Game/RefAssets/VIDAEnfermagem/Characters/Patient/BP_Patient.bAttachedToSyringe` _coletorreferencia_2)))
      (`self.MostraMãoAlgodão`)
      (set `/Game/RefAssets/VIDAEnfermagem/Characters/Patient/BP_Patient.bProcedureInProgress` false _coletorreferencia_2))))

(event `self.TriggerAlgodão.OnComponentEndOverlap`
  (params (OverlappedComponent :type "PrimitiveComponent Object Reference") (OtherActor :type "Actor Object Reference") (OtherComp :type "PrimitiveComponent Object Reference") (OtherBodyIndex :type Integer))
  (if (`KismetStringLibrary.EqualEqual_StrStr` (`KismetSystemLibrary.GetObjectName` OtherComp) "AlgodãoSeco")
    (`self.EscondeMãoAlgodão`)))

(fn `DefineAnimação`
  (locals (`ComeçouColeta` :type Boolean :default false) (PosicaoJogador :type "Vector Structure"))
  (bind _outactors (`GameplayStatics.GetAllActorsOfClass` null))
  (if (`HeadMountedDisplayFunctionLibrary.IsHeadMountedDisplayEnabled`)
    (bind _output (`|GetArrayItem` _outactors))
    (set `local.PosicaoJogador` (`SceneComponent.K2_GetComponentLocation` (`/Game/RefAssets/VIDAEnfermagem/Characters/Patient/BP_Patient.Camera` _output)))
    (else
      (set `local.PosicaoJogador` (`self.K2_GetActorLocation` _output))))
  (bind _outactors_2 (`GameplayStatics.GetAllActorsOfClass` null))
  (bind _output_2 (`|GetArrayItem` _outactors_2))
  (set `local.ComeçouColeta` (or (`self.naVeia`) (`/Game/RefAssets/VIDAEnfermagem/Characters/Patient/BP_Patient.noBraço` _output_2) (`self.Garroteado`)))
  (set `self.MaoFechada` (or (== _output_2 (`/Game/RefAssets/VIDAEnfermagem/Characters/Patient/BP_Patient.ObjetoAnexadoDireita` null)) (== _output_2 (`/Game/RefAssets/VIDAEnfermagem/Characters/Patient/BP_Patient.ObjetoAnexadoEsquerda` null)) (`local.ComeçouColeta`) (`self.Puxada`)))
  (set `self.Coletando` (or (`local.ComeçouColeta`) (<= (`self.CalculaDistancia` (`local.PosicaoJogador`) (`self.K2_GetActorLocation`)) 120.0)))
  (return))

(fn `DefineOpacidadeDecal`
  (locals (Max :type "Float (double-precision)") (Min :type "Float (double-precision)"))
  (bind _output_get (set `local.Max` 0.0))
  (if (`self.Puxada`)
    (bind _output_get_2 (set `local.Max` (+ _output_get 0.4))))
  (if (`self.Garroteado`)
    (bind _output_get_3 (set `local.Max` (+ _output_get_2 0.5))))
  (set `self.VeiasMaxDecalOpacity` _output_get_3)
  (bind _output_get_4 (set `local.Min` 0.9))
  (if (not (`self.Puxada`))
    (bind _output_get_5 (set `local.Min` (- _output_get_4 0.4))))
  (if (not (`self.Garroteado`))
    (bind _output_get_6 (set `local.Min` (- _output_get_5 0.5))))
  (set `self.VeiasMinDecalOpacity` _output_get_6)
  (return))

(fn `EscondeMãoAlgodão`
  (`SceneComponent.SetVisibility` (`self.AlgodaoSeco`) false false)
  (if (`SceneComponent.IsVisible` (`self.MaoEsquerdaAlgodaoSeco`))
    (`SceneComponent.SetVisibility` (`self.MaoEsquerdaAlgodaoSeco`) false false)
    (bind (_right _left) (`self.GetHandMeshes` (`.JogadorReferencia` (`self.JogadorReferencia`))))
    (`SceneComponent.SetVisibility` _left true true)
    (`self.SetarReferencias`)
    (else
      (`SceneComponent.SetVisibility` (`self.MaoDireitaAlgodaoSeco`) false false)
      (bind _right_2 (`self.GetHandMeshes` (`.JogadorReferencia` (`self.JogadorReferencia`))))
      (`SceneComponent.SetVisibility` _right_2 true true)
      (`self.SetarReferencias`))))

(fn `EscondeMãoDireitaPuxada`
  (if (`self.Puxada`)
    (set `self.FadeOutVeias` true)
    (bind _right (`self.GetHandMeshes` (`.JogadorReferencia` (`self.JogadorReferencia`))))
    (`SceneComponent.SetVisibility` _right true false)
    (`SceneComponent.SetVisibility` (`self.MaoDireitaPuxada`) false false)
    (set `self.Puxada` false)))

(fn `EscondeMãoEsquerdaPuxada`
  (if (`self.Puxada`)
    (set `self.FadeOutVeias` true)
    (bind (_right _left) (`self.GetHandMeshes` (`.JogadorReferencia` (`self.JogadorReferencia`))))
    (`SceneComponent.SetVisibility` _left true false)
    (`SceneComponent.SetVisibility` (`self.MaoEsquerdaPuxada`) false false)
    (set `self.Puxada` false)))

(fn `EsconderAssepsia`
  (bind _assepsiaopacity (`self.AssepsiaOpacity`))
  (if (<= _assepsiaopacity (`self.AssepsiaMinDecalOpacity`))
    (set `self.FadeOutAssepsia` false)
    (else
      (bind _output_get (set `self.AssepsiaOpacity` (- _assepsiaopacity (`self.AssepsiaFadeSpeed`))))
      (`MaterialInstanceDynamic.SetScalarParameterValue` (`self.AssepsiaDecalMaterial`) "Opacity" _output_get)))
  (return))

(fn `EsconderVeias`
  (bind _veiasopacity (`self.VeiasOpacity`))
  (if (<= _veiasopacity (`self.VeiasMinDecalOpacity`))
    (set `self.FadeOutVeias` false)
    (else
      (bind _output_get (set `self.VeiasOpacity` (- _veiasopacity (`self.VeiasFadeSpeed`))))
      (`MaterialInstanceDynamic.SetScalarParameterValue` (`self.DecalMaterial`) "Opacity" _output_get)))
  (return))

(fn `MostraMãoAlgodão`
  (bind (`_intermediário_referência` `_intermediário_referência_2`) (`self.Intermediário Referência`))
  (bind (`_intermediário_referência_3` `_intermediário_referência_4`) (`self.Intermediário Referência`))
  (bind (_jogadorreferencia _jogadorreferencia_2) (`self.JogadorReferencia`))
  (`SceneComponent.SetVisibility` (`self.AlgodaoSeco`) true false)
  (`SceneComponent.K2_SetWorldLocation` (`self.AlgodaoSeco`) (+ (`SceneComponent.K2_GetComponentLocation` (`/Game/RefAssets/VIDAEnfermagem/Characters/Patient/BP_Patient.Meia Ponta` (`.Intermediário Referência` (`self.Intermediário Referência`)))) (0.0 0.0 2.0)) false false)
  (set `/Game/RefAssets/VIDAEnfermagem/Characters/Patient/BP_Patient.ProcedimentoEmProgresso` false (`.Intermediário Referência` (`self.Intermediário Referência`)))
  (if (`/Game/RefAssets/VIDAEnfermagem/Characters/Patient/BP_Patient.ProcedimentoMaoDireita` `_intermediário_referência_2`)
    (`SceneComponent.SetVisibility` (`self.MaoEsquerdaAlgodaoSeco`) true false)
    (bind (_right _left) (`self.GetHandMeshes` _jogadorreferencia_2))
    (`SceneComponent.SetVisibility` _left false true)
    (`SceneComponent.SetVisibility` _right true true)
    (`SceneComponent.SetVisibility` (`/Game/RefAssets/VIDAEnfermagem/Characters/Patient/BP_Patient.SMPegouDireita` `_intermediário_referência_4`) false true)
    (elif (`/Game/RefAssets/VIDAEnfermagem/Characters/Patient/BP_Patient.ProcedimentoMaoEsquerda` `_intermediário_referência_2`)
      (`SceneComponent.SetVisibility` (`self.MaoDireitaAlgodaoSeco`) true false)
      (bind (_right_2 _left_2) (`self.GetHandMeshes` _jogadorreferencia_2))
      (`SceneComponent.SetVisibility` _right_2 false true)
      (`SceneComponent.SetVisibility` _left_2 true true)
      (`SceneComponent.SetVisibility` (`/Game/RefAssets/VIDAEnfermagem/Characters/Patient/BP_Patient.SMPegouEsquerda` `_intermediário_referência_4`) false true))))

(fn `MostraMãoDireitaPuxada`
  (set `self.FadeInVeias` true)
  (bind _right (`self.GetHandMeshes` (`.JogadorReferencia` (`self.JogadorReferencia`))))
  (`SceneComponent.SetVisibility` _right false false)
  (`SceneComponent.SetVisibility` (`self.MaoDireitaPuxada`) true false)
  (set `self.Puxada` true))

(fn `MostraMãoEsquerdaPuxada`
  (set `self.FadeInVeias` true)
  (bind (_right _left) (`self.GetHandMeshes` (`.JogadorReferencia` (`self.JogadorReferencia`))))
  (`SceneComponent.SetVisibility` _left false false)
  (`SceneComponent.SetVisibility` (`self.MaoEsquerdaPuxada`) true false)
  (set `self.Puxada` true))

(fn `MostrarAssepsia`
  (bind _assepsiaopacity (`self.AssepsiaOpacity`))
  (if (>= _assepsiaopacity (`self.AssepsiaMaxDecalOpacity`))
    (set `self.FadeInAssepsia` false)
    (else
      (bind _output_get (set `self.AssepsiaOpacity` (+ _assepsiaopacity (`self.AssepsiaFadeSpeed`))))
      (`MaterialInstanceDynamic.SetScalarParameterValue` (`self.AssepsiaDecalMaterial`) "Opacity" _output_get)))
  (return))

(fn `MostrarVeias`
  (bind _veiasopacity (`self.VeiasOpacity`))
  (if (>= _veiasopacity (`self.VeiasMaxDecalOpacity`))
    (set `self.FadeInVeias` false)
    (else
      (bind _output_get (set `self.VeiasOpacity` (+ _veiasopacity (`self.VeiasFadeSpeed`))))
      (`MaterialInstanceDynamic.SetScalarParameterValue` (`self.DecalMaterial`) "Opacity" _output_get)))
  (return))

(fn `PrenderGarroteNoBraço`
  (bind _asbp_floating_hands (cast `` (`GameplayStatics.GetPlayerCharacter` 0)))
  (bind (_success _tourniquet) (`self.SoltarGarroteDaMão` _asbp_floating_hands))
  (if _success
    (bind _rootcomponent (`Actor.RootComponent` _tourniquet))
    (`SceneComponent.SetVisibility` _rootcomponent true false)
    (set `self.GarroteReferência` null _tourniquet)
    (`SceneComponent.K2_SetWorldLocation` _rootcomponent (0.0 0.0 -20.0) false false)
    (`SceneComponent.SetVisibility` (`self.GarrotePreso`) true false)
    (set `self.Garroteado` true)
    (set `self.FadeInVeias` true)
    (`self.EscreveRelatorio` "Garroteou")
    (`self.PatientBuckled` (`.FSM` (`self.FSM`)))))

(fn `SetarReferencias`
  (bind _returnvalue (`KismetSystemLibrary.IsValid` (`.JogadorReferencia` (`self.JogadorReferencia`))))
  (bind _returnvalue_2 (`KismetSystemLibrary.IsValid` (`.GarroteReferência` (`self.GarroteReferência`))))
  (bind _returnvalue_3 (`KismetSystemLibrary.IsValid` (`.Intermediário Referência` (`self.Intermediário Referência`))))
  (bind _returnvalue_4 (`KismetSystemLibrary.IsValid` (`.ColetorReferencia` (`self.ColetorReferencia`))))
  (while (not (`self.ReferenciasSetadas`))
    (if (not _returnvalue)
      (bind _outactors (`GameplayStatics.GetAllActorsOfClass` null))
      (set `self.JogadorReferencia` null null))
    (if (not _returnvalue_2)
      (bind _outactors_2 (`GameplayStatics.GetAllActorsOfClass` null))
      (set `self.GarroteReferência` null null))
    (if _returnvalue_3
      (if (not _returnvalue_4)
        (bind _outactors_3 (`GameplayStatics.GetAllActorsOfClass` null :!label _label))
        (set `self.ColetorReferencia` null null))
      (else
        (bind _outactors_4 (`GameplayStatics.GetAllActorsOfClass` null))
        (set `self.Intermediário Referência` null null)
        (goto _label)))
    (set `self.ReferenciasSetadas` (and _returnvalue _returnvalue_2 _returnvalue_3 _returnvalue_4))))

(fn `setup`
  (bind _decalassepsia (`self.DecalAssepsia`))
  (bind _decalveia (`self.DecalVeia`))
  (`self.SetarReferencias`)
  (`SceneComponent.SetVisibility` (`self.GarrotePreso`) false false)
  (set `self.Garroteado` false)
  (bind _returnvalue (`KismetMaterialLibrary.CreateDynamicMaterialInstance` (`DecalComponent.GetDecalMaterial` _decalveia)))
  (bind _output_get (set `self.DecalMaterial` _returnvalue))
  (`DecalComponent.SetDecalMaterial` _decalveia _output_get)
  (bind _returnvalue_2 (`KismetMaterialLibrary.CreateDynamicMaterialInstance` (`DecalComponent.GetDecalMaterial` _decalassepsia)))
  (bind _output_get_2 (set `self.AssepsiaDecalMaterial` _returnvalue_2))
  (`DecalComponent.SetDecalMaterial` _decalassepsia _output_get_2)
  (cast `` (`GameplayStatics.GetGameMode`)))

(fn `SoltarGarroteDaMão`
  (params (In :type "Object Object Reference"))
  (returns (Success :type Boolean) (Tourniquet :type "Object Object Reference"))
  (if (`/Game/RefAssets/VIDAEnfermagem/Characters/Patient/BP_Patient.PegandoDireita` In)
    (bind _asbp_tourniquet_buckle (cast `` (`/Game/RefAssets/VIDAEnfermagem/Characters/Patient/BP_Patient.ObjetoAnexadoDireita` In))
      (:`then`
        (if (`/Game/RefAssets/VIDAEnfermagem/Characters/Patient/BP_Patient.bOverlappingPatient` _asbp_tourniquet_buckle)
          (`self.Soltar_D` In)
          (return true _asbp_tourniquet_buckle)
          (else
            (return false null))))
      (:`CastFailed`
        _)))
  (if (`/Game/RefAssets/VIDAEnfermagem/Characters/Patient/BP_Patient.PegandoEsquerda` In)
    (bind _asbp_tourniquet_buckle_2 (cast `` (`/Game/RefAssets/VIDAEnfermagem/Characters/Patient/BP_Patient.ObjetoAnexadoEsquerda` In)))
    (if (`/Game/RefAssets/VIDAEnfermagem/Characters/Patient/BP_Patient.bOverlappingPatient` _asbp_tourniquet_buckle_2)
      (`self.Soltar_E` In)
      (return true _asbp_tourniquet_buckle_2)
      (else
        (return false null)))))

(fn `SoltarGarroteDoBraço`
  (bind (_jogadorreferencia _jogadorreferencia_2) (`self.JogadorReferencia`))
  (bind (`_garrotereferência` `_garrotereferência_2`) (`self.GarroteReferência`))
  (bind _garrotepreso (`self.GarrotePreso`))
  (bind _asbp_floating_hands (cast `` (`GameplayStatics.GetPlayerCharacter` 0)))
  (if (`self.Garroteado`)
    (bind _asbp_custom_leap_low_poly_hand (cast `` (`ChildActorComponent.ChildActor` (`/Game/RefAssets/VIDAEnfermagem/Characters/Patient/BP_Patient.LeapHands` _asbp_floating_hands))))
    (if (and (not (`/Game/RefAssets/VIDAEnfermagem/Characters/Patient/BP_Patient.PegandoDireita` _asbp_floating_hands)) (`PrimitiveComponent.IsOverlappingComponent` (`/Game/RefAssets/VIDAEnfermagem/Characters/Patient/BP_Patient.Right` _asbp_custom_leap_low_poly_hand) _garrotepreso))
      (set `/Game/RefAssets/VIDAEnfermagem/Characters/Patient/BP_Patient.TocandoDireita` true _jogadorreferencia_2)
      (set `/Game/RefAssets/VIDAEnfermagem/Characters/Patient/BP_Patient.ObjetoTocandoDireita` `_garrotereferência_2` _jogadorreferencia_2)
      (`SceneComponent.SetVisibility` (`self.GarrotePreso`) false false :!label _label)
      (set `self.Garroteado` false)
      (set `self.FadeOutVeias` true)
      (`self.EscreveRelatorio` "Desgarroteou")
      (`self.Patient Unbuckled` (`.FSM` (`self.FSM`)))
      (elif (and (`PrimitiveComponent.IsOverlappingComponent` (`/Game/RefAssets/VIDAEnfermagem/Characters/Patient/BP_Patient.Left` _asbp_custom_leap_low_poly_hand) _garrotepreso) (not (`/Game/RefAssets/VIDAEnfermagem/Characters/Patient/BP_Patient.PegandoEsquerda` _asbp_floating_hands)))
        (set `/Game/RefAssets/VIDAEnfermagem/Characters/Patient/BP_Patient.TocandoEsquerda` true _jogadorreferencia_2)
        (set `/Game/RefAssets/VIDAEnfermagem/Characters/Patient/BP_Patient.ObjetoTocandoEsquerda` `_garrotereferência_2` _jogadorreferencia_2)
        (goto _label)))))

(fn `UserConstructionScript`)