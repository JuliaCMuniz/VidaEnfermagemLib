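; Pickable blood collection tube for a nursing procedure simulation with Leap Motion hands.
; Overlapping a syringe that is in the arm or vein attaches the tube; in the vein, it starts collecting.
; Each tick scales the blood mesh until full, at one-third speed while the patient's tourniquet is on.
; A full tube counts up/down flips to detect homogenization; milestones are written to the report and sent to the procedure FSM.
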(event `self.ReceiveBeginPlay`
  (`self.Setup`))

(event `self.ColisãoDoColetor.OnComponentBeginOverlap`
  (params (OverlappedComponent :type "PrimitiveComponent Object Reference") (OtherActor :type "Actor Object Reference") (OtherComp :type "PrimitiveComponent Object Reference") (OtherBodyIndex :type Integer) (bFromSweep :type Boolean) (SweepResult :type "HitResult Structure (by ref)"))
  (`self.AttachToSyringe` OtherActor OtherComp))

(event `self.ColisãoDoColetor.OnComponentEndOverlap`
  (params (OverlappedComponent :type "PrimitiveComponent Object Reference") (OtherActor :type "Actor Object Reference") (OtherComp :type "PrimitiveComponent Object Reference") (OtherBodyIndex :type Integer))
  (if (`KismetStringLibrary.EqualEqual_StrStr` "CorpoDoIntermediário" (`KismetSystemLibrary.GetObjectName` OtherComp))
    (set `self.bCollecting` false)))

(event `self.ReceiveTick`
  (params (DeltaSeconds :type "Float (single-precision)"))
  (`parent.ReceiveTick` DeltaSeconds)
  (`self.ScaleBloodIfCollecting`)
  (if (`self.bFull`)
    (`self.SetUpOrDown`))
  (if (`self.bAttachedToSyringe`)
    (cast `/Game/VIDAEnfermagem/Pickables/Syringe/BP_Syringe` (`ActorComponent.GetOwner` (`SceneComponent.GetAttachParent` (`self.RootComponent`)))
      (:`CastFailed`
        (set `self.bAttachedToSyringe` false)
        (bind _outactors (`GameplayStatics.GetAllActorsOfClass` "/Game/VIDAEnfermagem/Pickables/Syringe/BP_Syringe.BP_Syringe_C"))
        (set `/Game/VIDAEnfermagem/Pickables/Syringe/BP_Syringe.coletorAnexado` false (`|GetArrayItem` _outactors))))))

(fn `AttachToSyringe`
  (params (Actor :type "Actor Object Reference") (Componet :type "Object Object Reference"))
  (if (not (`self.bFull`))
    (bind _asbp_syringe (cast `/Game/VIDAEnfermagem/Pickables/Syringe/BP_Syringe` Actor))
    (if (or (`/Game/VIDAEnfermagem/Pickables/Syringe/BP_Syringe.naVeia` _asbp_syringe) (`/Game/VIDAEnfermagem/Pickables/Syringe/BP_Syringe.noBraço` _asbp_syringe))
      (`self.DetachFromHand`)
      (`SceneComponent.K2_AttachToComponent` (`self.RootComponent`) (`Actor.RootComponent` Actor) "None" "KeepRelative" "KeepRelative" "KeepRelative" true)
      (`self.K2_SetActorTransform` (`self.GetTransform` Actor))
      (if (`/Game/VIDAEnfermagem/Pickables/Syringe/BP_Syringe.naVeia` _asbp_syringe)
        (set `self.bCollecting` true)
        (`/Game/VIDAEnfermagem/Core/WriteText.EscreveRelatorio` "Anexou coletor")
        (`/Game/VIDAEnfermagem/Core/BP_ProcedureFSM.BloodCollectinStarted` (`self.FSM`))
        (set `self.bProcedureInProgress` true))
      (set `self.bAttachedToSyringe` true)
      (set `/Game/VIDAEnfermagem/Pickables/Syringe/BP_Syringe.coletorAnexado` true _asbp_syringe)
      (return))
    (else
      (return))))

(fn `DetachFromHand_0`
  (params (In :type "/Game/VIDAEnfermagem/Characters/Player/BP_FloatingHands Object Reference"))
  (if (`/Game/VIDAEnfermagem/Characters/Player/BP_FloatingHands.PegandoDireita` In)
    (if (`KismetStringLibrary.EqualEqual_StrStr` (`KismetSystemLibrary.GetClassDisplayName` (`GameplayStatics.GetObjectClass` (`/Game/VIDAEnfermagem/Characters/Player/BP_FloatingHands.ObjetoAnexadoDireita` In))) "Coletor_C")
      (`/Game/VIDAEnfermagem/Characters/Player/BP_FloatingHands.Soltar_D` In))
    (elif (`/Game/VIDAEnfermagem/Characters/Player/BP_FloatingHands.PegandoEsquerda` In)
      (if (`KismetStringLibrary.EqualEqual_StrStr` (`KismetSystemLibrary.GetClassDisplayName` (`GameplayStatics.GetObjectClass` (`/Game/VIDAEnfermagem/Characters/Player/BP_FloatingHands.ObjetoAnexadoEsquerda` In))) "Coletor_C")
        (`/Game/VIDAEnfermagem/Characters/Player/BP_FloatingHands.Soltar_E` In)))))

(fn `IsPickingEnabled`
  (returns (pegarAtivado :type Boolean))
  (bind _asbp_syringe (cast `/Game/VIDAEnfermagem/Pickables/Syringe/BP_Syringe` (`self.GetAttachParentActor` (`ActorComponent.GetOwner` (`self.RootComponent`))))
    (:`then`
      (for _array_element (`self.GetOverlappingActors` _asbp_syringe null)
        (cast `/Game/VIDAEnfermagem/Core/Leap/BP_CustomLeapLowPolyHand` _array_element)
        (if (`self.bCollecting`)
          (return false)
          (else
            (return true)))))
    (:`CastFailed`
      _))
  (return true))

(fn `ScaleBloodIfCollecting`
  (returns (coletorCheio :type Boolean))
  (bind _sangue (`self.Sangue`))
  (bind _bloodspeed (`self.BloodSpeed`))
  (bind _relativescale3d (`SceneComponent.RelativeScale3D` _sangue))
  (if (`self.bCollecting`)
    (`/Engine/EditorBlueprintResources/StandardMacros.CompareFloat` (.z _relativescale3d) 0.6
      (:`>`
        (bind _output_get (set `self.bCollecting` false :!label _label))
        (set `self.bFull` true)
        (`/Game/VIDAEnfermagem/Core/WriteText.EscreveRelatorio` "Coletor Cheio.")
        (`/Game/VIDAEnfermagem/Core/BP_ProcedureFSM.BloodCollected` (`self.FSM`))
        (return _output_get))
      (:`==`
        (goto _label))
      (:`<`
        (`SceneComponent.SetRelativeScale3D` _sangue (+ _relativescale3d (`KismetMathLibrary.MakeVector` 0.0 0.0 (select `bool` (`/Game/VIDAEnfermagem/Characters/Patient/BP_Patient.Garroteado` (`self.paciente`)) :`false` _bloodspeed :`true` (/ _bloodspeed 3.0)))))))))

(fn `SetReferences_0`
  (bind _returnvalue (`KismetSystemLibrary.IsValid` (`self.paciente`)))
  (while (not (`self.ReferenciasSetadas`))
    (if (not _returnvalue)
      (bind _outactors (`GameplayStatics.GetAllActorsOfClass` "/Game/VIDAEnfermagem/Characters/Patient/BP_Patient.BP_Patient_C"))
      (set `self.paciente` (`|GetArrayItem` _outactors)))
    (set `self.ReferenciasSetadas` _returnvalue)))

(fn `Setup`
  (bind (_transformpadrao_location _transformpadrao_rotation _transformpadrao_scale) (`KismetMathLibrary.BreakTransform` (`self.transformPadrao`)))
  (`parent.ReceiveBeginPlay`)
  (set `self.transformMaoDireita` (`KismetMathLibrary.MakeTransform` (-11.0 4.0 8.0) (struct :`Pitch` 110.0) _transformpadrao_scale))
  (set `self.transformMaoEsquerda` (`KismetMathLibrary.MakeTransform` (12.0 -4.0 -5.0) (struct :`Pitch` -80.0) _transformpadrao_scale))
  (`self.SetReferences_0`))

(fn `SetUpOrDown`
  (bind _z (.z (`KismetMathLibrary.Conv_RotatorToVector` (`SceneComponent.K2_GetComponentRotation` (`self.GeometryCache`)))))
  (if (not (`self.bHomogenized`))
    (set `self.PreviousPosition` (`self.NewPosition`))
    (if (>= _z 0.75)
      (set `self.NewPosition` "cima")
      (elif (<= _z -0.75)
        (set `self.NewPosition` "baixo")
        (else
          (return))))
    (if (not (`KismetStringLibrary.EqualEqual_StrStr` (`self.PreviousPosition`) (`self.NewPosition`)))
      (bind _output_get (set `self.HalfSpins` (+ (`self.HalfSpins`) 1.0)))
      (bind _output_get_2 (set `self.Spins` (`KismetMathLibrary.FFloor` (/ _output_get 2.0))))
      (if (>= _output_get_2 10)
        (set `self.bHomogenized` true)
        (`/Game/VIDAEnfermagem/Core/WriteText.EscreveRelatorio` "Homogeneizou amostra.")
        (`/Game/VIDAEnfermagem/Core/BP_ProcedureFSM.SampleHomogenized` (`self.FSM`))))
    (return)))

(fn `UserConstructionScript`)