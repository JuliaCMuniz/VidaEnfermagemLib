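; Pickable training cube that highlights itself when the tutorial reaches its cube-picking step.
; On BeginPlay it sets left and right hand transforms and applies a dynamic material to the mesh.
; Tick polls the TrainingFSM state, using DoOnce to start a green Glow timeline at Picking Cube and clear it at Picking Syringe.
; GetPegarAtivado allows pickup only from the Picking Cube state onward.
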(event `self.setarReferências`)

(event `self.ReceiveBeginPlay`
  (`self.setup`)
  (bind _returnvalue (`KismetMaterialLibrary.CreateDynamicMaterialInstance` "/Game/VIDAEnfermagem/MaterialLibrary/SimpleColors/M_LightGray.M_LightGray"))
  (bind _output_get (set `self.DynamicMaterial` _returnvalue))
  (`PrimitiveComponent.SetMaterial` (`self.Cube`) 0 _output_get))

(event `self.ReceiveTick`
  (params (DeltaSeconds :type "Float (single-precision)"))
  (bind _dynamicmaterial (`self.DynamicMaterial`))
  (`parent.ReceiveTick` DeltaSeconds)
  (switch `/Game/VIDAEnfermagem/Core/E_TrainingState` (`/Game/VIDAEnfermagem/Core/BP_TrainingFSM.State` (`self.TrainingFSM`))
    (:`NewEnumerator2`
      (`/Engine/EditorBlueprintResources/StandardMacros.DoOnce` false
        (:`Completed`
          (`MaterialInstanceDynamic.SetVectorParameterValue` _dynamicmaterial "color" (struct :`R` 0.074769 :`G` 1.0 :`A` 1.0))
          (bind (_direction _glow) (`Timeline|Glow` :`NewTime` DeltaSeconds :!via `PlayFromStart` :!label _label)
            (:`Update`
              (`MaterialInstanceDynamic.SetScalarParameterValue` (`self.DynamicMaterial`) "Brightness" _glow))))))
    (:`NewEnumerator3`
      (`/Engine/EditorBlueprintResources/StandardMacros.DoOnce` false
        (:`Completed`
          (`MaterialInstanceDynamic.SetVectorParameterValue` _dynamicmaterial "color" (struct :`R` 0.8 :`G` 0.8 :`B` 0.8 :`A` 1.0))
          (`|ExecutionSequence`
            (:`then_0`
              (goto _label :!via `Stop`))
            (:`then_1`
              (`MaterialInstanceDynamic.SetScalarParameterValue` (`self.DynamicMaterial`) "Brightness" 0.0))))))))

(fn `getPegarAtivado`
  (returns (pegarAtivado :type Boolean))
  (switch `/Game/VIDAEnfermagem/Core/E_TrainingState` (`/Game/VIDAEnfermagem/Core/BP_TrainingFSM.State` (`self.TrainingFSM`))
    (:`NewEnumerator8`
      _)
    (:`NewEnumerator9`
      _)
    (:`NewEnumerator0`
      _)
    (:`NewEnumerator1`
      _)
    (:`NewEnumerator10`
      _)
    (:`NewEnumerator2`
      (return true))
    (:`NewEnumerator3`
      (return true))
    (:`NewEnumerator4`
      (return true))
    (:`NewEnumerator7`
      (return true)))
  (return false))

(fn `setup`
  (bind (_transformpadrao_location _transformpadrao_rotation _transformpadrao_scale) (`KismetMathLibrary.BreakTransform` (`self.transformPadrao`)))
  (`parent.ReceiveBeginPlay`)
  (set `self.transformMaoDireita` (`KismetMathLibrary.MakeTransform` (-15.0 9.0 10.0) (struct) _transformpadrao_scale))
  (set `self.transformMaoEsquerda` (`KismetMathLibrary.MakeTransform` (16.0 -8.0 -8.5) (struct) _transformpadrao_scale)))

(fn `UserConstructionScript`)