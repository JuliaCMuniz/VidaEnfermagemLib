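; Nursing-sim supply tray that collects tourniquet, intermediary, collector, antiseptic cotton, dry cotton and needle.
; On box overlap, an attachment-parent check gates a cast chain that releases new items from the player's hand, snaps them to per-item transforms and logs each placement.
; Already-placed items only get TriggerBandeja set; end overlap clears it through a single cast.
; Setup sets hand transforms and finds the player; IsPickingEnabled returns false.
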(event `self.ReceiveBeginPlay`
  (`self.setup`))

(event `self.ReceiveTick`
  (params (DeltaSeconds :type "Float (double-precision)")))

(event `self.Box.OnComponentBeginOverlap`
  (params (OverlappedComponent :type "PrimitiveComponent Object Reference") (OtherActor :type "Actor Object Reference") (OtherComp :type "PrimitiveComponent Object Reference") (OtherBodyIndex :type Integer) (bFromSweep :type Boolean) (SweepResult :type "HitResult Structure (by ref)"))
  (bind _keeprelative (`self.KeepRelative`))
  (bind _transformpadraoagulha (`self.TransformPadraoAgulha`))
  (bind _transformpadraogarrote (`self.TransformPadraoGarrote`))
  (bind _transformpadraointermediario (`self.TransformPadraoIntermediario`))
  (bind _transformpadraocoletor (`self.TransformPadraoColetor`))
  (bind _transformpadraoalgodaoantisseptico (`self.TransformPadraoAlgodaoAntisseptico`))
  (bind _keeprelative_2 (`self.KeepRelative`))
  (bind _keeprelative_3 (`self.KeepRelative`))
  (bind _keeprelative_4 (`self.KeepRelative`))
  (bind _keeprelative_5 (`self.KeepRelative`))
  (bind _keeprelative_6 (`self.KeepRelative`))
  (bind _transformpadraoalgodaoseco (`self.TransformPadraoAlgodaoSeco`))
  (bind _returnvalue (`self.GetAttachParentActor` (`ActorComponent.GetOwner` (`Actor.RootComponent` OtherActor))))
  (cast `` _returnvalue
    (:`then`
      _)
    (:`CastFailed`
      (cast `` _returnvalue)))
  (bind _asbp_tourniquet_buckle (cast `` OtherActor)
    (:`then`
      (if (`/Game/RefAssets/VIDAEnfermagem/Pickables/Tray/BP_Tray.FoiColocadoNaBandeja` _asbp_tourniquet_buckle)
        (set `/Game/RefAssets/VIDAEnfermagem/Pickables/Tray/BP_Tray.triggerBandeja` true _asbp_tourniquet_buckle)
        (else
          (`self.SoltarDaMão_0` _asbp_tourniquet_buckle)
          (`self.K2_AttachToActor` _asbp_tourniquet_buckle self "None" _keeprelative _keeprelative _keeprelative true)
          (`self.K2_SetActorRelativeTransform` _asbp_tourniquet_buckle _transformpadraogarrote false false)
          (set `/Game/RefAssets/VIDAEnfermagem/Pickables/Tray/BP_Tray.transformPadrao` _transformpadraogarrote _asbp_tourniquet_buckle)
          (set `/Game/RefAssets/VIDAEnfermagem/Pickables/Tray/BP_Tray.FoiColocadoNaBandeja` true _asbp_tourniquet_buckle)
          (`self.EscreveRelatorio` "Colocou  Garrote na Bandeja"))))
    (:`CastFailed`
      (bind _asbp_syringe (cast `` OtherActor)
        (:`then`
          (if (`/Game/RefAssets/VIDAEnfermagem/Pickables/Tray/BP_Tray.FoiColocadoNaBandeja` _asbp_syringe)
            (set `/Game/RefAssets/VIDAEnfermagem/Pickables/Tray/BP_Tray.triggerBandeja` true _asbp_syringe)
            (else
              (`self.SoltarDaMão_0` _asbp_syringe)
              (`self.K2_AttachToActor` _asbp_syringe self "None" _keeprelative_3 _keeprelative_3 _keeprelative_3 true)
              (`self.K2_SetActorRelativeTransform` _asbp_syringe _transformpadraointermediario false false)
              (set `/Game/RefAssets/VIDAEnfermagem/Pickables/Tray/BP_Tray.transformPadrao` _transformpadraointermediario _asbp_syringe)
              (set `/Game/RefAssets/VIDAEnfermagem/Pickables/Tray/BP_Tray.FoiColocadoNaBandeja` true _asbp_syringe)
              (`self.EscreveRelatorio` "Colocou  Intermediario na Bandeja"))))
        (:`CastFailed`
          (bind _asbp_collection_tube (cast `` OtherActor)
            (:`then`
              (if (`/Game/RefAssets/VIDAEnfermagem/Pickables/Tray/BP_Tray.FoiColocadoNaBandeja` _asbp_collection_tube)
                (set `/Game/RefAssets/VIDAEnfermagem/Pickables/Tray/BP_Tray.triggerBandeja` true _asbp_collection_tube)
                (else
                  (`self.SoltarDaMão_0` _asbp_collection_tube)
                  (`self.K2_AttachToActor` _asbp_collection_tube self "None" _keeprelative_5 _keeprelative_5 _keeprelative_5 true)
                  (`self.K2_SetActorRelativeTransform` _asbp_collection_tube _transformpadraocoletor false false)
                  (set `/Game/RefAssets/VIDAEnfermagem/Pickables/Tray/BP_Tray.transformPadrao` _transformpadraocoletor _asbp_collection_tube)
                  (set `/Game/RefAssets/VIDAEnfermagem/Pickables/Tray/BP_Tray.FoiColocadoNaBandeja` true _asbp_collection_tube)
                  (`self.EscreveRelatorio` "Colocou  Coletor na Bandeja"))))
            (:`CastFailed`
              (bind _asbp_cotton_wet (cast `` OtherActor)
                (:`then`
                  (if (`/Game/RefAssets/VIDAEnfermagem/Pickables/Tray/BP_Tray.FoiColocadoNaBandeja` _asbp_cotton_wet)
                    (set `/Game/RefAssets/VIDAEnfermagem/Pickables/Tray/BP_Tray.triggerBandeja` true _asbp_cotton_wet)
                    (else
                      (`self.SoltarDaMão_0` _asbp_cotton_wet)
                      (`self.K2_AttachToActor` _asbp_cotton_wet self "None" _keeprelative_6 _keeprelative_6 _keeprelative_6 true)
                      (`self.K2_SetActorRelativeTransform` _asbp_cotton_wet _transformpadraoalgodaoantisseptico false false)
                      (set `/Game/RefAssets/VIDAEnfermagem/Pickables/Tray/BP_Tray.transformPadrao` _transformpadraoalgodaoantisseptico _asbp_cotton_wet)
                      (set `/Game/RefAssets/VIDAEnfermagem/Pickables/Tray/BP_Tray.FoiColocadoNaBandeja` true _asbp_cotton_wet)
                      (`self.EscreveRelatorio` "Colocou  Algodão Antisséptic na Bandeja"))))
                (:`CastFailed`
                  (bind _asbp_cotton_dry (cast `` OtherActor)
                    (:`then`
                      (if (`/Game/RefAssets/VIDAEnfermagem/Pickables/Tray/BP_Tray.FoiColocadoNaBandeja` _asbp_cotton_dry)
                        (set `/Game/RefAssets/VIDAEnfermagem/Pickables/Tray/BP_Tray.triggerBandeja` true _asbp_cotton_dry)
                        (else
                          (`self.SoltarDaMão_0` _asbp_cotton_dry)
                          (`self.K2_AttachToActor` _asbp_cotton_dry self "None" _keeprelative_4 _keeprelative_4 _keeprelative_4 true)
                          (`self.K2_SetActorRelativeTransform` _asbp_cotton_dry _transformpadraoalgodaoseco false false)
                          (set `/Game/RefAssets/VIDAEnfermagem/Pickables/Tray/BP_Tray.transformPadrao` _transformpadraoalgodaoseco _asbp_cotton_dry)
                          (set `/Game/RefAssets/VIDAEnfermagem/Pickables/Tray/BP_Tray.FoiColocadoNaBandeja` true _asbp_cotton_dry)
                          (`self.EscreveRelatorio` "Colocou  Algodão Seco na Bandeja"))))
                    (:`CastFailed`
                      (bind _asbp_needle (cast `` OtherActor))
                      (if (`/Game/RefAssets/VIDAEnfermagem/Pickables/Tray/BP_Tray.FoiColocadoNaBandeja` _asbp_needle)
                        (set `/Game/RefAssets/VIDAEnfermagem/Pickables/Tray/BP_Tray.triggerBandeja` true _asbp_needle)
                        (else
                          (`self.SoltarDaMão_0` _asbp_needle)
                          (`self.K2_AttachToActor` _asbp_needle self "None" _keeprelative_2 _keeprelative_2 _keeprelative_2 true)
                          (`self.K2_SetActorRelativeTransform` _asbp_needle _transformpadraoagulha false false)
                          (set `/Game/RefAssets/VIDAEnfermagem/Pickables/Tray/BP_Tray.transformPadrao` _transformpadraoagulha _asbp_needle)
                          (set `/Game/RefAssets/VIDAEnfermagem/Pickables/Tray/BP_Tray.FoiColocadoNaBandeja` true _asbp_needle)
                          (`self.EscreveRelatorio` "Colocou  Agulha na Bandeja"))))))))))))))

(event `self.Box.OnComponentEndOverlap`
  (params (OverlappedComponent :type "PrimitiveComponent Object Reference") (OtherActor :type "Actor Object Reference") (OtherComp :type "PrimitiveComponent Object Reference") (OtherBodyIndex :type Integer))
  (bind _asbp_pickable_object (cast `` OtherActor))
  (set `/Game/RefAssets/VIDAEnfermagem/Pickables/Tray/BP_Tray.triggerBandeja` false _asbp_pickable_object))

(fn `IsPickingEnabled`
  (returns (pegarAtivado :type Boolean))
  (return false))

(fn `SetarReferencias`
  (bind _returnvalue (`KismetSystemLibrary.IsValid` (`self.JogadorReferencia`)))
  (while (not (`self.ReferenciasSetadas`))
    (if (not _returnvalue)
      (bind _outactors (`GameplayStatics.GetAllActorsOfClass` null))
      (set `self.JogadorReferencia` (`|GetArrayItem` _outactors)))
    (set `self.ReferenciasSetadas` _returnvalue)))

(fn `setup`
  (bind (_transformpadrao_location _transformpadrao_rotation _transformpadrao_scale) (`KismetMathLibrary.BreakTransform` (`self.transformPadrao`)))
  (set `self.transformMaoDireita` (`KismetMathLibrary.MakeTransform` (-22.48 16.57 14.89) (struct :`Pitch` 27.440001 :`Yaw` 104.519997 :`Roll` -8.91) _transformpadrao_scale))
  (set `self.transformMaoEsquerda` (`KismetMathLibrary.MakeTransform` (20.741327 -23.360912 -5.805843) (struct :`Yaw` 97.186996 :`Roll` 158.389999) _transformpadrao_scale))
  (`self.SetarReferencias`))

(fn `SoltarDaMão_0`
  (params (ObjetoPegavel :type "Object Object Reference"))
  (bind _jogadorreferencia (`self.JogadorReferencia`))
  (if (`/Game/RefAssets/VIDAEnfermagem/Pickables/Tray/BP_Tray.PegandoDireita` _jogadorreferencia)
    (if (`KismetStringLibrary.EqualEqual_StrStr` (`KismetSystemLibrary.GetDisplayName` (`/Game/RefAssets/VIDAEnfermagem/Pickables/Tray/BP_Tray.ObjetoAnexadoDireita` _jogadorreferencia)) (`KismetSystemLibrary.GetDisplayName` ObjetoPegavel))
      (`self.Soltar_D` _jogadorreferencia)
      (else
        (if (`/Game/RefAssets/VIDAEnfermagem/Pickables/Tray/BP_Tray.PegandoEsquerda` _jogadorreferencia) :!label _label
          (if (`KismetStringLibrary.EqualEqual_StrStr` (`KismetSystemLibrary.GetDisplayName` ObjetoPegavel) (`KismetSystemLibrary.GetDisplayName` (`/Game/RefAssets/VIDAEnfermagem/Pickables/Tray/BP_Tray.ObjetoAnexadoEsquerda` _jogadorreferencia)))
            (`self.Soltar_E` _jogadorreferencia)))))
    (else
      (goto _label))))

(fn `UserConstructionScript`)