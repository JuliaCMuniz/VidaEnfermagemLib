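; VR training syringe that glows during the pick-up step and ends the tutorial when its tip pierces the target Sphere.
; While inside, it locks rotation and slides along the entry axis, projecting palm movement onto it (ProdutoVetorial is a dot product), capped at maximum depth.
; A ghost hand replaces the player's hand until exit restores the grip transform.
; TrainingFSM state drives the timeline highlight and gates grabbing.
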(event `self.ReceiveBeginPlay`
  (`self.setup`)
  (bind _returnvalue (`KismetMaterialLibrary.CreateDynamicMaterialInstance` "/Game/VIDAEnfermagem/MaterialLibrary/SimpleColors/M_LightGray.M_LightGray"))
  (bind _output_get (set `self.Dynamic Material` _returnvalue))
  (`PrimitiveComponent.SetMaterial` (`self.Cylinder`) 0 _output_get))

(event `self.ponta.OnComponentBeginOverlap`
  (params (OverlappedComponent :type "PrimitiveComponent Object Reference") (OtherActor :type "Actor Object Reference") (OtherComp :type "PrimitiveComponent Object Reference") (OtherBodyIndex :type Integer) (bFromSweep :type Boolean) (SweepResult :type "HitResult Structure (by ref)"))
  (bind _trainingfsm (`self.TrainingFSM`))
  (if (`KismetStringLibrary.EqualEqual_StrStr` (`KismetSystemLibrary.GetObjectName` OtherComp) "Sphere")
    (set `self.noBraço` true)
    (bind `_posiçãopalma` (`self.PegaPosições`))
    (set `self.PosiçãoInicial` `_posiçãopalma`)
    (set `self.VetorUnitarioEntrada` (`self.CalculaVetorUnitario`))
    (set `self.RotaçãoPerfuração` (`self.K2_GetActorRotation`))
    (set `self.PosiçãoPerfuração` (`self.K2_GetActorLocation`))
    (`self.MostrarMãoFantasma`)
    (switch `/Game/VIDAEnfermagem/Core/E_TrainingState` (`/Game/VIDAEnfermagem/Core/BP_TrainingFSM.State` _trainingfsm)
      (:`NewEnumerator4`
        (set `/Game/VIDAEnfermagem/Core/BP_TrainingFSM.State` "NewEnumerator7" _trainingfsm)))))

(event `self.ponta.OnComponentEndOverlap`
  (params (OverlappedComponent :type "PrimitiveComponent Object Reference") (OtherActor :type "Actor Object Reference") (OtherComp :type "PrimitiveComponent Object Reference") (OtherBodyIndex :type Integer))
  (if (`KismetStringLibrary.EqualEqual_StrStr` (`KismetSystemLibrary.GetObjectName` OtherComp) "Sphere")
    (set `self.noBraço` false)
    (`self.EsconderMãoFantasma`)
    (bind _newparam (`self.isAttachedToRight`))
    (if _newparam
      (`self.K2_SetActorRelativeTransform` (`self.transformMaoDireita`))
      (else
        (`self.K2_SetActorRelativeTransform` (`self.transformMaoEsquerda`))))))

(event `self.ReceiveTick`
  (params (DeltaSeconds :type "Float (single-precision)"))
  (bind _dynamic_material (`self.Dynamic Material`))
  (bind _profundidademaxima (`self.ProfundidadeMaxima`))
  (bind _vetorunitarioentrada (`self.VetorUnitarioEntrada`))
  (if (`self.noBraço`)
    (bind `_posiçãopalma` (`self.PegaPosições`))
    (bind _returnvalue (/ (`self.ProdutoVetorial` (- (`self.PosiçãoInicial`) `_posiçãopalma`) _vetorunitarioentrada) (`self.ProdutoVetorial` _vetorunitarioentrada _vetorunitarioentrada)))
    (if (> _profundidademaxima _returnvalue)
      (set `self.Profundidade` _returnvalue)
      (else
        (set `self.Profundidade` _profundidademaxima)))
    (`self.K2_SetActorLocationAndRotation` (- (`self.PosiçãoPerfuração`) (* (`self.VetorUnitarioEntrada`) (`self.Profundidade`))) (`self.RotaçãoPerfuração`))
    (else
      (switch `/Game/VIDAEnfermagem/Core/E_TrainingState` (`/Game/VIDAEnfermagem/Core/BP_TrainingFSM.State` (`self.TrainingFSM`))
        (:`NewEnumerator3`
          (`/Engine/EditorBlueprintResources/StandardMacros.DoOnce` false
            (:`Completed`
              (`MaterialInstanceDynamic.SetVectorParameterValue` _dynamic_material "color" (struct :`R` 0.074769 :`G` 1.0 :`A` 1.0))
              (bind (_direction _glow) (`Timeline|Timeline_1` :!via `PlayFromStart` :!label _label)
                (:`Update`
                  (`MaterialInstanceDynamic.SetScalarParameterValue` (`self.Dynamic Material`) "Brightness" _glow))))))
        (:`NewEnumerator4`
          (`/Engine/EditorBlueprintResources/StandardMacros.DoOnce` false
            (:`Completed`
              (`MaterialInstanceDynamic.SetVectorParameterValue` _dynamic_material "color" (struct :`R` 0.8 :`G` 0.8 :`B` 0.8 :`A` 1.0))
              (`|ExecutionSequence`
                (:`then_0`
                  (goto _label :!via `Stop`))
                (:`then_1`
                  (`MaterialInstanceDynamic.SetScalarParameterValue` (`self.Dynamic Material`) "Brightness" 0.0))))))))))

(fn `EsconderMãoFantasma`
  (bind _jogadorreferencia (`self.JogadorReferencia`))
  (bind _newparam (`self.isAttachedToRight`))
  (if _newparam
    (bind _right (`/Game/VIDAEnfermagem/Characters/Player/BP_FloatingHands_Training.GetHandMeshes` _jogadorreferencia))
    (`SceneComponent.SetVisibility` _right true false)
    (`SceneComponent.SetVisibility` (`self.SMPegouDireita`) false false)
    (else
      (bind (_right_2 _left) (`/Game/VIDAEnfermagem/Characters/Player/BP_FloatingHands_Training.GetHandMeshes` _jogadorreferencia))
      (`SceneComponent.SetVisibility` _left true false)
      (`SceneComponent.SetVisibility` (`self.SMPegouEsquerda`) false false))))

(fn `getPegarAtivado`
  (returns (pegarAtivado :type Boolean))
  (switch `/Game/VIDAEnfermagem/Core/E_TrainingState` (`/Game/VIDAEnfermagem/Core/BP_TrainingFSM.State` (`self.TrainingFSM`))
    (:`NewEnumerator0`
      _)
    (:`NewEnumerator1`
      _)
    (:`NewEnumerator2`
      _)
    (:`NewEnumerator3`
      (return true))
    (:`NewEnumerator4`
      (return true))
    (:`NewEnumerator7`
      (return true)))
  (return false))

(fn `MostrarMãoFantasma`
  (bind _jogadorreferencia (`self.JogadorReferencia`))
  (bind _newparam (`self.isAttachedToRight`))
  (if _newparam
    (bind _right (`/Game/VIDAEnfermagem/Characters/Player/BP_FloatingHands_Training.GetHandMeshes` _jogadorreferencia))
    (`SceneComponent.SetVisibility` _right false false)
    (`SceneComponent.SetVisibility` (`self.SMPegouDireita`) true false)
    (else
      (bind (_right_2 _left) (`/Game/VIDAEnfermagem/Characters/Player/BP_FloatingHands_Training.GetHandMeshes` _jogadorreferencia))
      (`SceneComponent.SetVisibility` _left false false)
      (`SceneComponent.SetVisibility` (`self.SMPegouEsquerda`) true false))))

(fn `PegaPosições`
  (returns (`PosiçãoPalma` :type "Vector Structure"))
  (bind _returnvalue (`ActorComponent.GetOwner` (`self.RootComponent`)))
  (bind _rootcomponent (`Actor.RootComponent` _returnvalue))
  (bind _returnvalue_2 (`KismetStringLibrary.Conv_NameToString` (`self.GetAttachParentSocketName` _returnvalue)))
  (bind _returnvalue_location (`KismetMathLibrary.BreakTransform` (`SceneComponent.GetSocketTransform` _rootcomponent "R_Palm" "RTS_World")))
  (bind _returnvalue_location_2 (`KismetMathLibrary.BreakTransform` (`SceneComponent.GetSocketTransform` _rootcomponent "L_Palm" "RTS_World")))
  (if (`KismetStringLibrary.EqualEqual_StrStr` "R_Palm" _returnvalue_2)
    (return _returnvalue_location)
    (elif (`KismetStringLibrary.EqualEqual_StrStr` "L_Palm" _returnvalue_2)
      (return _returnvalue_location_2))))

(fn `setup`
  (bind (_transformpadrao_location _transformpadrao_rotation _transformpadrao_scale) (`KismetMathLibrary.BreakTransform` (`self.transformPadrao`)))
  (`parent.ReceiveBeginPlay`)
  (`self.SetTickGroup` "TG_PostUpdateWork")
  (set `self.transformMaoDireita` (`KismetMathLibrary.MakeTransform` (-10.0 4.5 5.0) (struct :`Pitch` 160.0) _transformpadrao_scale))
  (set `self.transformMaoEsquerda` (`KismetMathLibrary.MakeTransform` (11.59 -3.23 -3.4) (struct :`Pitch` -38.049999 :`Yaw` 10.91 :`Roll` 4.3) _transformpadrao_scale))
  (bind _outactors (`GameplayStatics.GetAllActorsOfClass` "/Game/VIDAEnfermagem/Characters/Player/BP_FloatingHands_Training.BP_FloatingHands_Training_C"))
  (set `self.JogadorReferencia` (`|GetArrayItem` _outactors)))

(fn `UserConstructionScript`)