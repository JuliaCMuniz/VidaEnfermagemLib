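; Demo syringe pickable for a nursing venipuncture simulation, held by Leap Motion hands and inserted into a patient's arm.
; On arm contact it records the entry pose and swaps the hand for a ghost mesh.
; Tick projects palm movement onto the needle axis, locking the syringe to that line with capped depth and releasing it on withdrawal.
; The tip reports vein hits to the game mode, and numpad 4/6 rotate the bevel.
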(event `self.ReceiveBeginPlay`
  (`self.setup`))

(event `Key|NumPadFour` :consume false
  (params (Key :type "Key Structure"))
  (bind _returnvalue (`SceneComponent.GetAttachParent` (`self.RootComponent`)))
  ;[1 1 1] Ajuste do bizel
  (:`Pressed`
    (`/Engine/EditorBlueprintResources/StandardMacros.IsValid` _returnvalue
      (:`Is Valid`
        (if (`.bSuccess` (cast `/Game/VIDAEnfermagem/Core/Leap/BP_CustomLeapLowPolyHand` (`ActorComponent.GetOwner` _returnvalue) :!pure true))
          (set `self.girarEsquerda` true)
          (set `self.deltaRotação` (struct :`Roll` -5.0))))))
  (:`Released`
    (set `self.girarEsquerda` false)))

(event `Key|NumPadSix` :consume false
  (params (Key :type "Key Structure"))
  (bind _returnvalue (`SceneComponent.GetAttachParent` (`self.RootComponent`)))
  ;[1 1 1] Ajuste do bizel
  (:`Pressed`
    (`/Engine/EditorBlueprintResources/StandardMacros.IsValid` _returnvalue
      (:`Is Valid`
        (if (`.bSuccess` (cast `/Game/VIDAEnfermagem/Core/Leap/BP_CustomLeapLowPolyHand` (`ActorComponent.GetOwner` _returnvalue) :!pure true))
          (set `self.girarDireita` true)
          (set `self.deltaRotação` (struct :`Roll` 5.0))))))
  (:`Released`
    (set `self.girarDireita` false)))

(event `self.Cylinder.OnComponentBeginOverlap`
  (params (OverlappedComponent :type "PrimitiveComponent Object Reference") (OtherActor :type "Actor Object Reference") (OtherComp :type "PrimitiveComponent Object Reference") (OtherBodyIndex :type Integer) (bFromSweep :type Boolean) (SweepResult :type "HitResult Structure (by ref)"))
  (if (`KismetStringLibrary.EqualEqual_StrStr` (`KismetSystemLibrary.GetObjectName` OtherComp) "remy")
    (if (not (`self.noBraço`))
      (set `self.noBraço` true)
      (bind `_posiçãopalma` (`self.PegaPosições`))
      (set `self.PosiçãoInicial` `_posiçãopalma`)
      (set `self.VetorUnitarioEntrada` (`self.CalculaVetorUnitario`))
      (set `self.RotaçãoPerfuração` (`self.K2_GetActorRotation`))
      (set `self.PosiçãoPerfuração` (`self.K2_GetActorLocation`))
      (`self.MostrarMãoFantasma`))))

(event `self.Ponta.OnComponentBeginOverlap`
  (params (OverlappedComponent :type "PrimitiveComponent Object Reference") (OtherActor :type "Actor Object Reference") (OtherComp :type "PrimitiveComponent Object Reference") (OtherBodyIndex :type Integer) (bFromSweep :type Boolean) (SweepResult :type "HitResult Structure (by ref)"))
  (if (`ActorComponent.ComponentHasTag` OtherComp "Veia")
    (set `self.naVeia` true)
    (bind _asdemo_gamemode (cast `/Game/VIDAEnfermagem/Core/Demo_Gamemode` (`GameplayStatics.GetGameMode`)))
    (`/Game/VIDAEnfermagem/Core/Demo_Gamemode.displayEvent` _asdemo_gamemode 5.0 "Acertou veia!")))

(event `self.Ponta.OnComponentEndOverlap`
  (params (OverlappedComponent :type "PrimitiveComponent Object Reference") (OtherActor :type "Actor Object Reference") (OtherComp :type "PrimitiveComponent Object Reference") (OtherBodyIndex :type Integer))
  (if (`ActorComponent.ComponentHasTag` OtherComp "Veia")
    (set `self.naVeia` false)
    (bind _asdemo_gamemode (cast `/Game/VIDAEnfermagem/Core/Demo_Gamemode` (`GameplayStatics.GetGameMode`)))
    (`/Game/VIDAEnfermagem/Core/Demo_Gamemode.clearEvent` _asdemo_gamemode)))

(event `self.ReceiveTick`
  (params (DeltaSeconds :type "Float (single-precision)"))
  (bind _profundidademaxima (`self.ProfundidadeMaxima`))
  (bind _vetorunitarioentrada (`self.VetorUnitarioEntrada`))
  (`parent.ReceiveTick` DeltaSeconds)
  (if (`self.referenciasSetadas`)
    (bind (`_posiçãopalma` `_rotaçãopalma`) (`self.PegaPosições`))
    (set `self.coletorAnexado` (`/Game/VIDAEnfermagem/Pickables/CollectionTube/BP_CollectionTube_Demo.noIntermediário` (`self.coletor`)))
    (if (and (`self.noBraço`) true (`SceneComponent.IsVisible` (`self.P4-2`)))
      (set `self.Rotação` (`self.ProdutoVetorial` (`KismetMathLibrary.Conv_RotatorToVector` `_rotaçãopalma`) (`KismetMathLibrary.Conv_RotatorToVector` (`self.RotaçãoPerfuração`))))
      (bind _returnvalue (/ (`self.ProdutoVetorial` (- (`self.PosiçãoInicial`) `_posiçãopalma`) _vetorunitarioentrada) (`self.ProdutoVetorial` _vetorunitarioentrada _vetorunitarioentrada)))
      (if (> _profundidademaxima _returnvalue)
        (if (>= _returnvalue (`self.ProfundidadeMinima`))
          (set `self.Profundidade` _returnvalue)
          (`self.AplicaConstraint` :!label _label)
          (`self.AjustaBizel` :!label _label_2)
          (else
            (set `self.noBraço` false)
            (bind _true (`self.isAttachedToRight`))
            (if _true
              (`self.K2_SetActorRelativeTransform` (`self.transformMaoDireita`))
              (else
                (`self.K2_SetActorRelativeTransform` (`self.transformMaoEsquerda`))))
            (`self.EsconderMãoFantasma`)))
        (else
          (set `self.Profundidade` _profundidademaxima)
          (goto _label)))
      (else
        (goto _label_2)))))

(fn `AjustaBizel`
  (if (xor (`self.girarEsquerda`) (`self.girarDireita`))
    (if (`self.girarEsquerda`)
      (`SceneComponent.K2_AddLocalRotation` (`self.Scene`) (struct :`Roll` -0.5) false false)
      (elif (`self.girarDireita`)
        (`SceneComponent.K2_AddLocalRotation` (`self.Scene`) (struct :`Roll` 0.5) false false)))))

(fn `AplicaConstraint`
  (`self.K2_SetActorLocationAndRotation` (- (`self.PosiçãoPerfuração`) (* (`self.VetorUnitarioEntrada`) (`self.Profundidade`))) (`self.RotaçãoPerfuração`)))

(fn `CalculaProfundidade`
  (locals (NewLocalVar_0 :type "/Game/VIDAEnfermagem/Core/BP_PickableObject Object Reference"))
  (bind _profundidademaxima (`self.ProfundidadeMaxima`))
  (bind _vetorunitarioentrada (`self.VetorUnitarioEntrada`))
  (bind `_posiçãopalma` (`self.PegaPosições`))
  (bind _returnvalue (/ (`self.ProdutoVetorial` (- (`self.PosiçãoInicial`) `_posiçãopalma`) _vetorunitarioentrada) (`self.ProdutoVetorial` _vetorunitarioentrada _vetorunitarioentrada)))
  (if (> _profundidademaxima _returnvalue)
    (if (>= _returnvalue (`self.ProfundidadeMinima`))
      (set `self.Profundidade` _returnvalue)
      (return)
      (else
        (set `self.noBraço` false)
        (`self.K2_SetActorRelativeTransform` (`self.transformMaoDireita`))
        (`self.EsconderMãoFantasma`)))
    (else
      (set `self.Profundidade` _profundidademaxima)
      (return))))

(fn `EsconderMãoFantasma`
  (bind `_jogador_referência` (`self.Jogador Referência`))
  (bind _true (`self.isAttachedToRight`))
  (if _true
    (bind _right (`/Game/VIDAEnfermagem/Characters/Player/BP_FloatingHands_Demo.GetHandMeshes` `_jogador_referência`))
    (`SceneComponent.SetVisibility` _right true false)
    (`SceneComponent.SetVisibility` (`self.SMPegouDireita`) false false)
    (else
      (bind (_right_2 _left) (`/Game/VIDAEnfermagem/Characters/Player/BP_FloatingHands_Demo.GetHandMeshes` `_jogador_referência`))
      (`SceneComponent.SetVisibility` _left true false)
      (`SceneComponent.SetVisibility` (`self.SMPegouEsquerda`) false false))))

(fn `IsPickingEnabled`
  (returns (pegarAtivado :type Boolean))
  (return (and (not (`self.ProcedimentoEmProgresso`)) (not (`self.coletorAnexado`)) (not (`self.esquerdaSegurando`)) (`/Game/VIDAEnfermagem/Core/Demo_Gamemode.Começou` (cast `/Game/VIDAEnfermagem/Core/Demo_Gamemode` (`GameplayStatics.GetGameMode`) :!pure true)))))

(fn `MostrarMãoFantasma`
  (bind `_jogador_referência` (`self.Jogador Referência`))
  (bind _true (`self.isAttachedToRight`))
  (if _true
    (bind _right (`/Game/VIDAEnfermagem/Characters/Player/BP_FloatingHands_Demo.GetHandMeshes` `_jogador_referência`))
    (`SceneComponent.SetVisibility` _right false false)
    (`SceneComponent.SetVisibility` (`self.SMPegouDireita`) true false)
    (else
      (bind (_right_2 _left) (`/Game/VIDAEnfermagem/Characters/Player/BP_FloatingHands_Demo.GetHandMeshes` `_jogador_referência`))
      (`SceneComponent.SetVisibility` _left false false)
      (`SceneComponent.SetVisibility` (`self.SMPegouEsquerda`) true false))))

(fn `PegaPosições`
  (returns (`PosiçãoPalma` :type "Vector Structure") (`RotaçãoPalma` :type "Rotator Structure"))
  (bind _returnvalue (`ActorComponent.GetOwner` (`self.RootComponent`)))
  (bind _returnvalue_2 (`KismetStringLibrary.Conv_NameToString` (`self.GetAttachParentSocketName` _returnvalue)))
  (bind _asbp_custom_leap_low_poly_hand (cast `/Game/VIDAEnfermagem/Core/Leap/BP_CustomLeapLowPolyHand` (`self.GetAttachParentActor` _returnvalue) :!pure true))
  (bind (_returnvalue_location _returnvalue_rotation) (`KismetMathLibrary.BreakTransform` (`SceneComponent.GetSocketTransform` (`/Game/VIDAEnfermagem/Core/Leap/BP_CustomLeapLowPolyHand.Right` _asbp_custom_leap_low_poly_hand) "R_Palm" "RTS_World")))
  (bind (_returnvalue_location_2 _returnvalue_rotation_2) (`KismetMathLibrary.BreakTransform` (`SceneComponent.GetSocketTransform` (`/Game/VIDAEnfermagem/Core/Leap/BP_CustomLeapLowPolyHand.Left` _asbp_custom_leap_low_poly_hand) "L_Palm" "RTS_World")))
  (if (`KismetStringLibrary.EqualEqual_StrStr` "R_Palm" _returnvalue_2)
    (return _returnvalue_location _returnvalue_rotation)
    (elif (`KismetStringLibrary.EqualEqual_StrStr` "L_Palm" _returnvalue_2)
      (return _returnvalue_location_2 _returnvalue_rotation_2))))

(fn `ResetarReferencias`
  (bind _returnvalue (`KismetSystemLibrary.IsValid` (`self.Jogador Referência`)))
  (bind _returnvalue_2 (`KismetSystemLibrary.IsValid` (`self.paciente`)))
  (bind _returnvalue_3 (`KismetSystemLibrary.IsValid` (`self.coletor`)))
  (while (not (`self.referenciasSetadas`))
    (if (not _returnvalue)
      (bind _outactors (`GameplayStatics.GetAllActorsOfClass` "/Game/VIDAEnfermagem/Characters/Player/BP_FloatingHands_Demo.BP_FloatingHands_Demo_C"))
      (set `self.Jogador Referência` (`|GetArrayItem` _outactors)))
    (if (not _returnvalue_2)
      (bind _outactors_2 (`GameplayStatics.GetAllActorsOfClass` "/Game/VIDAEnfermagem/Characters/Patient/BP_Patient_Demo.BP_Patient_Demo_C"))
      (set `self.paciente` (`|GetArrayItem` _outactors_2)))
    (if (not _returnvalue_3)
      (bind _outactors_3 (`GameplayStatics.GetAllActorsOfClass` "/Game/VIDAEnfermagem/Pickables/CollectionTube/BP_CollectionTube_Demo.BP_CollectionTube_Demo_C"))
      (set `self.coletor` (`|GetArrayItem` _outactors_3)))
    (set `self.referenciasSetadas` (and _returnvalue _returnvalue_2 _returnvalue_3))))

(fn `setup`
  (bind (_transformpadrao_location _transformpadrao_rotation _transformpadrao_scale) (`KismetMathLibrary.BreakTransform` (`self.transformPadrao`)))
  (`self.SetTickGroup` "TG_PostUpdateWork")
  (`parent.ReceiveBeginPlay`)
  (set `self.transformMaoDireita` (`KismetMathLibrary.MakeTransform` (-10.0 4.5 5.0) (struct :`Pitch` 160.0) _transformpadrao_scale))
  (set `self.transformMaoEsquerda` (`KismetMathLibrary.MakeTransform` (11.59 -3.23 -3.4) (struct :`Pitch` -38.049999 :`Yaw` 10.91 :`Roll` 4.3) _transformpadrao_scale))
  (`self.ResetarReferencias`))

(fn `UserConstructionScript`)