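; Pickable syringe for a hand-tracked nursing blood-collection simulation, reporting mounting, puncture and withdrawal steps to the procedure FSM.
; Overlapping a held needle mounts it, while tip overlaps detect patient and vein punctures.
; Once in the arm, Tick projects palm movement onto the entry vector to constrain depth at fixed rotation, releasing below minimum.
; Ghost hand meshes replace tracked hands during the procedure, and numpad 4/6 rotate the bevel.
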(event `Key|NumPadFour` :consume false
  (params (Key :type "Key Structure"))
  (bind _returnvalue (`SceneComponent.GetAttachParent` (`self.RootComponent`)))
  ;[1 1 1] Ajuste do bizel
  (:`Pressed`
    (`/Engine/EditorBlueprintResources/StandardMacros.IsValid` _returnvalue
      (:`Is Valid`
        (if (`.bSuccess` (cast `/Game/VIDAEnfermagem/Core/Leap/BP_CustomLeapLowPolyHand` (`ActorComponent.GetOwner` _returnvalue) :!pure true))
          (set `self.girarEsquerda` true)
          (set `self.deltaRotação` (struct :`Roll` -5.0))))))
  (:`Released`
    (set `self.girarEsquerda` false)))

(event `Key|NumPadSix` :consume false
  (params (Key :type "Key Structure"))
  (bind _returnvalue (`SceneComponent.GetAttachParent` (`self.RootComponent`)))
  ;[1 1 1] Ajuste do bizel
  (:`Pressed`
    (`/Engine/EditorBlueprintResources/StandardMacros.IsValid` _returnvalue
      (:`Is Valid`
        (if (`.bSuccess` (cast `/Game/VIDAEnfermagem/Core/Leap/BP_CustomLeapLowPolyHand` (`ActorComponent.GetOwner` _returnvalue) :!pure true))
          (set `self.girarDireita` true)
          (set `self.deltaRotação` (struct :`Roll` 5.0))))))
  (:`Released`
    (set `self.girarDireita` false)))

(event `self.ReceiveBeginPlay`
  (`self.setup`))

(event `self.Ponta.OnComponentBeginOverlap`
  (params (OverlappedComponent :type "PrimitiveComponent Object Reference") (OtherActor :type "Actor Object Reference") (OtherComp :type "PrimitiveComponent Object Reference") (OtherBodyIndex :type Integer) (bFromSweep :type Boolean) (SweepResult :type "HitResult Structure (by ref)"))
  (bind `_nobraço` (`self.noBraço`))
  (if (`KismetStringLibrary.EqualEqual_StrStr` (`KismetSystemLibrary.GetObjectName` OtherComp) "remy")
    (`/Game/VIDAEnfermagem/Core/BP_ProcedureFSM.PatientPunctured` (`self.FSM`))
    (if (not `_nobraço`)
      (set `self.noBraço` true)
      (bind `_posiçãopalma` (`self.PegaPosições`))
      (set `self.PosiçãoInicial` `_posiçãopalma`)
      (set `self.VetorUnitarioEntrada` (`self.CalculaVetorUnitario`))
      (set `self.RotaçãoPerfuração` (`self.K2_GetActorRotation`))
      (set `self.PosiçãoPerfuração` (`self.K2_GetActorLocation`))
      (`self.MostrarMãoFantasma`)
      (`/Game/VIDAEnfermagem/Core/WriteText.EscreveRelatorio` (`KismetStringLibrary.Concat_StrStr` "Perfurou Paciente, Rotação: " (`KismetStringLibrary.Conv_RotatorToString` (`self.K2_GetActorRotation`)))))
    (elif (and `_nobraço` (`ActorComponent.ComponentHasTag` OtherComp "Veia"))
      (bind _output_get (set `self.naVeia` true))
      (set `self.ProcedimentoEmProgresso` _output_get)
      (bind _newparam (`self.IsAttachedToRight`))
      (if _newparam
        (set `self.ProcedimentoMaoDireita` true)
        (else
          (set `self.ProcedimentoMaoEsquerda` true)))
      (set `PrimitiveComponent.bGenerateOverlapEvents` true (`self.Capsule`))
      (`/Game/VIDAEnfermagem/Core/WriteText.EscreveRelatorio` (`KismetStringLibrary.Concat_StrStr` "Perfurou Veia, Rotação: " (`KismetStringLibrary.Conv_RotatorToString` (`self.K2_GetActorRotation`))))
      (`/Game/VIDAEnfermagem/Core/BP_ProcedureFSM.VeinPunctured` (`self.FSM`)))))

(event `self.Ponta.OnComponentEndOverlap`
  (params (OverlappedComponent :type "PrimitiveComponent Object Reference") (OtherActor :type "Actor Object Reference") (OtherComp :type "PrimitiveComponent Object Reference") (OtherBodyIndex :type Integer))
  (if (`ActorComponent.ComponentHasTag` OtherComp "Veia")
    (bind _output_get (set `self.naVeia` false))
    (bind _output_get_2 (set `self.ProcedimentoEmProgresso` _output_get))
    (set `PrimitiveComponent.bGenerateOverlapEvents` _output_get_2 (`self.Capsule`))
    (bind _newparam (`self.IsAttachedToRight`))
    (if _newparam
      (set `self.ProcedimentoMaoDireita` false)
      (else
        (set `self.ProcedimentoMaoEsquerda` false)))
    (`/Game/VIDAEnfermagem/Core/BP_ProcedureFSM.VeinDepunctured` (`self.FSM`))))

(event `self.ReceiveTick`
  (params (DeltaSeconds :type "Float (single-precision)"))
  (bind _profundidademaxima (`self.ProfundidadeMaxima`))
  (bind _vetorunitarioentrada (`self.VetorUnitarioEntrada`))
  (`parent.ReceiveTick` DeltaSeconds)
  (if (`self.referenciasSetadas`)
    (set `self.coletorAnexado` (`/Game/VIDAEnfermagem/Pickables/CollectionTube/BP_CollectionTube.bAttachedToSyringe` (`self.coletor`)))
    (if (and (`self.noBraço`) true (`SceneComponent.IsVisible` (`self.P4-2`)))
      (bind (`_posiçãopalma` `_rotaçãopalma`) (`self.PegaPosições`))
      (set `self.Rotação` (`self.ProdutoVetorial` (`KismetMathLibrary.Conv_RotatorToVector` `_rotaçãopalma`) (`KismetMathLibrary.Conv_RotatorToVector` (`self.RotaçãoPerfuração`))))
      (bind _returnvalue (/ (`self.ProdutoVetorial` (- (`self.PosiçãoInicial`) `_posiçãopalma`) _vetorunitarioentrada) (`self.ProdutoVetorial` _vetorunitarioentrada _vetorunitarioentrada)))
      (if (> _profundidademaxima _returnvalue)
        (if (>= _returnvalue (`self.ProfundidadeMinima`))
          (set `self.Profundidade` _returnvalue)
          (`self.AplicaConstraint` :!label _label)
          (`self.AjustaBizel` :!label _label_2)
          (else
            (set `self.noBraço` false)
            (bind _newparam (`self.IsAttachedToRight`))
            (if _newparam
              (`self.K2_SetActorRelativeTransform` (`self.transformMaoDireita`))
              (else
                (`self.K2_SetActorRelativeTransform` (`self.transformMaoEsquerda`))))
            (`self.EsconderMãoFantasma`)
            (`/Game/VIDAEnfermagem/Core/BP_ProcedureFSM.PatientDepunctured` (`self.FSM`))))
        (else
          (set `self.Profundidade` _profundidademaxima)
          (goto _label)))
      (else
        (goto _label_2)))
    (else
      (`self.ResetarReferencias`))))

(event `self.Capsule.OnComponentBeginOverlap`
  (params (OverlappedComponent :type "PrimitiveComponent Object Reference") (OtherActor :type "Actor Object Reference") (OtherComp :type "PrimitiveComponent Object Reference") (OtherBodyIndex :type Integer) (bFromSweep :type Boolean) (SweepResult :type "HitResult Structure (by ref)"))
  (bind _returnvalue (`KismetSystemLibrary.GetObjectName` OtherComp))
  (bind _procedimentoemprogresso (`self.ProcedimentoEmProgresso`))
  (if (`self.referenciasSetadas`)
    (if (and (`KismetStringLibrary.EqualEqual_StrStr` _returnvalue "Right") (== (`/Game/VIDAEnfermagem/Characters/Player/BP_FloatingHands.ObjetoAnexadoDireita` (`self.Jogador Referência`)) null) _procedimentoemprogresso (`self.ProcedimentoMaoDireita`))
      (bind _right (`/Game/VIDAEnfermagem/Characters/Player/BP_FloatingHands.GetHandMeshes` (`self.Jogador Referência`)))
      (`SceneComponent.SetVisibility` _right false false)
      (`SceneComponent.SetVisibility` (`self.SMPegouDireita`) true false)
      (elif (and (`KismetStringLibrary.EqualEqual_StrStr` _returnvalue "Left") _procedimentoemprogresso (`self.ProcedimentoMaoEsquerda`) (== (`/Game/VIDAEnfermagem/Characters/Player/BP_FloatingHands.ObjetoAnexadoEsquerda` (`self.Jogador Referência`)) null))
        (bind (_right_2 _left) (`/Game/VIDAEnfermagem/Characters/Player/BP_FloatingHands.GetHandMeshes` (`self.Jogador Referência`)))
        (`SceneComponent.SetVisibility` _left false false)
        (`SceneComponent.SetVisibility` (`self.SMPegouEsquerda`) true false)))))

(event `self.Capsule.OnComponentEndOverlap`
  (params (OverlappedComponent :type "PrimitiveComponent Object Reference") (OtherActor :type "Actor Object Reference") (OtherComp :type "PrimitiveComponent Object Reference") (OtherBodyIndex :type Integer))
  (bind _returnvalue (`KismetSystemLibrary.GetObjectName` OtherComp))
  (bind _procedimentoemprogresso (`self.ProcedimentoEmProgresso`))
  (if (and (`KismetStringLibrary.EqualEqual_StrStr` _returnvalue "Right") (== (`/Game/VIDAEnfermagem/Characters/Player/BP_FloatingHands.ObjetoAnexadoDireita` (`self.Jogador Referência`)) null) _procedimentoemprogresso (`self.ProcedimentoMaoDireita`))
    (bind _right (`/Game/VIDAEnfermagem/Characters/Player/BP_FloatingHands.GetHandMeshes` (`self.Jogador Referência`)))
    (`SceneComponent.SetVisibility` _right true false)
    (`SceneComponent.SetVisibility` (`self.SMPegouDireita`) false false)
    (elif (and (`KismetStringLibrary.EqualEqual_StrStr` _returnvalue "Left") _procedimentoemprogresso (== (`/Game/VIDAEnfermagem/Characters/Player/BP_FloatingHands.ObjetoAnexadoEsquerda` (`self.Jogador Referência`)) null) (`self.ProcedimentoMaoEsquerda`))
      (bind (_right_2 _left) (`/Game/VIDAEnfermagem/Characters/Player/BP_FloatingHands.GetHandMeshes` (`self.Jogador Referência`)))
      (`SceneComponent.SetVisibility` _left true false)
      (`SceneComponent.SetVisibility` (`self.SMPegouEsquerda`) false false))))

(event `self.Intermediario-2.OnComponentBeginOverlap`
  (params (OverlappedComponent :type "PrimitiveComponent Object Reference") (OtherActor :type "Actor Object Reference") (OtherComp :type "PrimitiveComponent Object Reference") (OtherBodyIndex :type Integer) (bFromSweep :type Boolean) (SweepResult :type "HitResult Structure (by ref)"))
  (bind _asbp_needle (cast `/Game/VIDAEnfermagem/Pickables/Syringe/BP_Needle` OtherActor))
  (cast `/Game/VIDAEnfermagem/Core/Leap/BP_CustomLeapLowPolyHand` (`self.GetAttachParentActor` (`ActorComponent.GetOwner` (`Actor.RootComponent` _asbp_needle))))
  (if true
    (`self.DetachFromHand` _asbp_needle)
    (`self.K2_AttachToActor` _asbp_needle self "None" "KeepRelative" "KeepRelative" "KeepRelative" true)
    (`self.SetActorHiddenInGame` OtherActor true)
    (`self.SetActorEnableCollision` _asbp_needle false)
    (`SceneComponent.SetVisibility` (`self.P4-2`) true true)
    (set `/Game/VIDAEnfermagem/Core/BP_PickableObject.pegarAtivado` true (cast `/Game/VIDAEnfermagem/Pickables/Syringe/BP_Protector` (`ChildActorComponent.ChildActor` (`self.Protetor`)) :!pure true))
    (`/Game/VIDAEnfermagem/Core/WriteText.EscreveRelatorio` "Intermediário Montado")
    (`/Game/VIDAEnfermagem/Core/BP_ProcedureFSM.SyringeMounted` (`self.FSM`))))

(fn `AjustaBizel`
  (if (xor (`self.girarEsquerda`) (`self.girarDireita`))
    (if (`self.girarEsquerda`)
      (`SceneComponent.K2_AddLocalRotation` (`self.Scene`) (struct :`Roll` -0.5) false false)
      (elif (`self.girarDireita`)
        (`SceneComponent.K2_AddLocalRotation` (`self.Scene`) (struct :`Roll` 0.5) false false)))))

(fn `AplicaConstraint`
  (`self.K2_SetActorLocationAndRotation` (- (`self.PosiçãoPerfuração`) (* (`self.VetorUnitarioEntrada`) (`self.Profundidade`))) (`self.RotaçãoPerfuração`)))

(fn `CalculaProfundidade`
  (locals (NewLocalVar_0 :type "/Game/VIDAEnfermagem/Core/BP_PickableObject Object Reference"))
  (bind _profundidademaxima (`self.ProfundidadeMaxima`))
  (bind _vetorunitarioentrada (`self.VetorUnitarioEntrada`))
  (bind `_posiçãopalma` (`self.PegaPosições`))
  (bind _returnvalue (/ (`self.ProdutoVetorial` (- (`self.PosiçãoInicial`) `_posiçãopalma`) _vetorunitarioentrada) (`self.ProdutoVetorial` _vetorunitarioentrada _vetorunitarioentrada)))
  (if (> _profundidademaxima _returnvalue)
    (if (>= _returnvalue (`self.ProfundidadeMinima`))
      (set `self.Profundidade` _returnvalue)
      (return)
      (else
        (set `self.noBraço` false)
        (`self.K2_SetActorRelativeTransform` (`self.transformMaoDireita`))
        (`self.EsconderMãoFantasma`)
        (`KismetSystemLibrary.PrintString` "Hello" true true (struct :`R` 1.0 :`B` 0.069903 :`A` 1.0))))
    (else
      (set `self.Profundidade` _profundidademaxima)
      (return))))

(fn `EsconderMãoFantasma`
  (bind `_jogador_referência` (`self.Jogador Referência`))
  (switch `/Game/VIDAEnfermagem/Core/E_ProcedureState` (`/Game/VIDAEnfermagem/Core/BP_ProcedureFSM.State` (`self.FSM`))
    (:`NewEnumerator0`
      (bind _newparam (`self.IsAttachedToRight` :!label _label))
      (if _newparam
        (bind _right (`/Game/VIDAEnfermagem/Characters/Player/BP_FloatingHands.GetHandMeshes` `_jogador_referência` :!label _label_2))
        (`SceneComponent.SetVisibility` _right true false)
        (`SceneComponent.SetVisibility` (`self.SMPegouDireita`) false false)
        (else
          (bind (_right_2 _left) (`/Game/VIDAEnfermagem/Characters/Player/BP_FloatingHands.GetHandMeshes` `_jogador_referência` :!label _label_3))
          (`SceneComponent.SetVisibility` _left true false)
          (`SceneComponent.SetVisibility` (`self.SMPegouEsquerda`) false false))))
    (:`NewEnumerator1`
      (goto _label))
    (:`NewEnumerator3`
      (goto _label))
    (:`NewEnumerator2`
      (goto _label))
    (:`NewEnumerator4`
      (goto _label))
    (:`NewEnumerator5`
      (goto _label))
    (:`NewEnumerator6`
      (goto _label))
    (:`NewEnumerator7`
      (goto _label))
    (:`NewEnumerator9`
      (goto _label))
    (:`NewEnumerator8`
      (goto _label))
    (:`NewEnumerator10`
      (if (`self.ProcedimentoMaoDireita`)
        (goto _label_3)
        (else
          (goto _label_2))))))

(fn `IsPickingEnabled`
  (returns (pegarAtivado :type Boolean))
  (return (and (not (`self.ProcedimentoEmProgresso`)) (not (`self.coletorAnexado`)) (not (`self.esquerdaSegurando`)))))

(fn `MostrarMãoFantasma`
  (bind `_jogador_referência` (`self.Jogador Referência`))
  (bind _newparam (`self.IsAttachedToRight`))
  (if _newparam
    (bind _right (`/Game/VIDAEnfermagem/Characters/Player/BP_FloatingHands.GetHandMeshes` `_jogador_referência`))
    (`SceneComponent.SetVisibility` _right false false)
    (`SceneComponent.SetVisibility` (`self.SMPegouDireita`) true false)
    (else
      (bind (_right_2 _left) (`/Game/VIDAEnfermagem/Characters/Player/BP_FloatingHands.GetHandMeshes` `_jogador_referência`))
      (`SceneComponent.SetVisibility` _left false false)
      (`SceneComponent.SetVisibility` (`self.SMPegouEsquerda`) true false))))

(fn `PegaPosições`
  (returns (`PosiçãoPalma` :type "Vector Structure") (`RotaçãoPalma` :type "Rotator Structure"))
  (bind _returnvalue (`ActorComponent.GetOwner` (`self.RootComponent`)))
  (bind _returnvalue_2 (`KismetStringLibrary.Conv_NameToString` (`self.GetAttachParentSocketName` _returnvalue)))
  (bind _asbp_custom_leap_low_poly_hand (cast `/Game/VIDAEnfermagem/Core/Leap/BP_CustomLeapLowPolyHand` (`self.GetAttachParentActor` _returnvalue) :!pure true))
  (bind (_returnvalue_location _returnvalue_rotation) (`KismetMathLibrary.BreakTransform` (`SceneComponent.GetSocketTransform` (`/Game/VIDAEnfermagem/Core/Leap/BP_CustomLeapLowPolyHand.Right` _asbp_custom_leap_low_poly_hand) "R_Palm" "RTS_World")))
  (bind (_returnvalue_location_2 _returnvalue_rotation_2) (`KismetMathLibrary.BreakTransform` (`SceneComponent.GetSocketTransform` (`/Game/VIDAEnfermagem/Core/Leap/BP_CustomLeapLowPolyHand.Left` _asbp_custom_leap_low_poly_hand) "L_Palm" "RTS_World")))
  (if (`KismetStringLibrary.EqualEqual_StrStr` "R_Palm" _returnvalue_2)
    (return _returnvalue_location _returnvalue_rotation)
    (elif (`KismetStringLibrary.EqualEqual_StrStr` "L_Palm" _returnvalue_2)
      (return _returnvalue_location_2 _returnvalue_rotation_2))))

(fn `ResetarReferencias`
  (bind _returnvalue (`KismetSystemLibrary.IsValid` (`self.Jogador Referência`)))
  (bind _returnvalue_2 (`KismetSystemLibrary.IsValid` (`self.paciente`)))
  (bind _returnvalue_3 (`KismetSystemLibrary.IsValid` (`self.coletor`)))
  (while (not (`self.referenciasSetadas`))
    (if (not _returnvalue)
      (bind _outactors (`GameplayStatics.GetAllActorsOfClass` "/Game/VIDAEnfermagem/Characters/Player/BP_FloatingHands.BP_FloatingHands_C"))
      (set `self.Jogador Referência` (`|GetArrayItem` _outactors)))
    (if (not _returnvalue_2)
      (bind _outactors_2 (`GameplayStatics.GetAllActorsOfClass` "/Game/VIDAEnfermagem/Characters/Patient/BP_Patient.BP_Patient_C"))
      (set `self.paciente` (`|GetArrayItem` _outactors_2)))
    (if (not _returnvalue_3)
      (bind _outactors_3 (`GameplayStatics.GetAllActorsOfClass` "/Game/VIDAEnfermagem/Pickables/CollectionTube/BP_CollectionTube.BP_CollectionTube_C"))
      (set `self.coletor` (`|GetArrayItem` _outactors_3)))
    (set `self.referenciasSetadas` (and _returnvalue _returnvalue_2 _returnvalue_3))))

(fn `SetarReferencias`
  (bind _outactors (`GameplayStatics.GetAllActorsOfClass` "/Game/VIDAEnfermagem/Characters/Player/BP_FloatingHands.BP_FloatingHands_C"))
  (set `self.Jogador Referência` (`|GetArrayItem` _outactors))
  (bind _outactors_2 (`GameplayStatics.GetAllActorsOfClass` "/Game/VIDAEnfermagem/Characters/Patient/BP_Patient.BP_Patient_C"))
  (set `self.paciente` (`|GetArrayItem` _outactors_2))
  (bind _outactors_3 (`GameplayStatics.GetAllActorsOfClass` "/Game/VIDAEnfermagem/Pickables/CollectionTube/BP_CollectionTube.BP_CollectionTube_C"))
  (set `self.coletor` (`|GetArrayItem` _outactors_3)))

(fn `setup`
  (bind (_transformpadrao_location _transformpadrao_rotation _transformpadrao_scale) (`KismetMathLibrary.BreakTransform` (`self.transformPadrao`)))
  (`self.SetTickGroup` "TG_PostUpdateWork")
  (`parent.ReceiveBeginPlay`)
  (set `self.transformMaoDireita` (`KismetMathLibrary.MakeTransform` (-10.0 4.5 5.0) (struct :`Pitch` 160.0) _transformpadrao_scale))
  (set `self.transformMaoEsquerda` (`KismetMathLibrary.MakeTransform` (11.59 -3.23 -3.4) (struct :`Pitch` -38.049999 :`Yaw` 10.91 :`Roll` 4.3) _transformpadrao_scale))
  (`self.SetarReferencias`))

(fn `UserConstructionScript`)