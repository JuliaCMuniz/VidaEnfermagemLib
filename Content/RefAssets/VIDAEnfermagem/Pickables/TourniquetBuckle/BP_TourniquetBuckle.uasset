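; BP_TourniquetBuckle is a pickable tourniquet buckle that knows when it overlaps a patient.
; On BeginPlay, Setup runs the parent's BeginPlay, then sets right-hand and left-hand transforms with fixed offsets and rotations, keeping the default transform's scale.
; Begin and end overlap events with BP_Patient toggle the OverlappingPatient flag.
; Tick only defers to the parent, followed by an empty branch.
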(event `self.ReceiveBeginPlay`
  (`self.setup`))

(event `self.ReceiveTick`
  (params (DeltaSeconds :type "Float (single-precision)"))
  (`parent.ReceiveTick` DeltaSeconds)
  (if true
    _))

(event `self.ReceiveActorBeginOverlap`
  (params (OtherActor :type "Actor Object Reference"))
  (cast `/Game/VIDAEnfermagem/Characters/Patient/BP_Patient` OtherActor)
  (set `self.bOverlappingPatient` true))

(event `self.ReceiveActorEndOverlap`
  (params (OtherActor :type "Actor Object Reference"))
  (cast `/Game/VIDAEnfermagem/Characters/Patient/BP_Patient` OtherActor)
  (set `self.bOverlappingPatient` false))

(fn `setup`
  (bind (_transformpadrao_location _transformpadrao_rotation _transformpadrao_scale) (`KismetMathLibrary.BreakTransform` (`self.transformPadrao`)))
  (`parent.ReceiveBeginPlay`)
  (set `self.transformMaoDireita` (`KismetMathLibrary.MakeTransform` (-9.0 8.0 2.0) (struct :`Pitch` 100.0) _transformpadrao_scale))
  (set `self.transformMaoEsquerda` (`KismetMathLibrary.MakeTransform` (10.0 -7.0 -2.0) (struct :`Pitch` -90.0 :`Yaw` 180.0) _transformpadrao_scale)))

(fn `UserConstructionScript`)