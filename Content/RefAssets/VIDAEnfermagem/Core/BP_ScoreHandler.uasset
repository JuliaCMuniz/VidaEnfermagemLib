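; BP_ScoreHandler is an actor that tracks a score and applies penalties for faults of three severities.
; Weak, medium and serious fault events each subtract a progressively larger amount from Score and print a Portuguese label naming the severity.
; A serious fault also calls Failure on the FSM reference, while lighter faults only lower the score, with no threshold check.
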(event `Weak Fault`
  (set `self.Score` (- (`self.Score`) 5))
  (`KismetSystemLibrary.PrintString` "Falha Leve" true true (struct :`R` 1.0 :`G` 0.015237 :`A` 1.0)))

(event `Medium Fault`
  (set `self.Score` (- (`self.Score`) 20))
  (`KismetSystemLibrary.PrintString` "Falha Média" true true (struct :`R` 1.0 :`G` 0.015237 :`A` 1.0)))

(event `Serious fault`
  (set `self.Score` (- (`self.Score`) 75))
  (`/Game/VIDAEnfermagem/Core/BP_ProcedureFSM.Failure` (`self.FSM`))
  (`KismetSystemLibrary.PrintString` "Falha Grave" true true (struct :`R` 1.0 :`G` 0.015237 :`A` 1.0)))

(fn `UserConstructionScript`)