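; Blueprint state machine for a nursing blood collection procedure, tracking the current step from putting on glasses to the end.
; Step events set completion flags and advance State based on the previous state, sometimes skipping steps already done.
; Out-of-order or missed steps report weak, medium or serious faults to ScoreHandler, and Failure forces the Fail state.
; Tick prints current and previous states on screen for debugging.
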(event `self.ReceiveTick`
  (params (DeltaSeconds :type "Float (single-precision)"))
  (`KismetSystemLibrary.PrintString` (`|GetEnumeratorNameAsString` (`self.State`)) true false (struct :`G` 0.66 :`B` 1.0 :`A` 1.0) DeltaSeconds)
  (`KismetSystemLibrary.PrintString` (`|GetEnumeratorNameAsString` (`self.PreviousState`)) true true (struct :`R` 0.040045 :`G` 1.0 :`A` 1.0) DeltaSeconds))

(event `self.ReceiveBeginPlay`
  (bind _output_get (set `self.State` "NewEnumerator0"))
  (set `self.PreviousState` _output_get))

(event `GlassesPutOn`
  (set `self.bGlassesPutOn` true)
  (bind _output_get (set `self.PreviousState` (`self.State`)))
  (switch `/Game/VIDAEnfermagem/Core/E_ProcedureState` _output_get
    (:`NewEnumerator0`
      (set `self.State` "NewEnumerator1"))))

(event `HandsWashed`
  (set `self.bHandsWashed` true)
  (bind _output_get (set `self.PreviousState` (`self.State`)))
  (switch `/Game/VIDAEnfermagem/Core/E_ProcedureState` _output_get
    (:`NewEnumerator1`
      (if (`self.bPatientBuckled`)
        (if (`self.bPatientSterilyzed`)
          (if (`self.bSyringeMounted`)
            (set `self.State` "NewEnumerator5")
            (else
              (set `self.State` "NewEnumerator4")))
          (else
            (set `self.State` "NewEnumerator2")))
        (else
          (set `self.State` "NewEnumerator3"))))))

(event `PatientSterilyzed`
  (set `self.bPatientSterilyzed` true)
  (bind _output_get (set `self.PreviousState` (`self.State`)))
  (switch `/Game/VIDAEnfermagem/Core/E_ProcedureState` _output_get
    (:`NewEnumerator2`
      (if (`self.bSyringeMounted`)
        (set `self.State` "NewEnumerator5")
        (`/Game/VIDAEnfermagem/Core/BP_ScoreHandler.Medium Fault` (`self.ScoreHandler`))
        (else
          (set `self.State` "NewEnumerator4"))))))

(event `PatientBuckled`
  (set `self.bPatientBuckled` true)
  (bind _output_get (set `self.PreviousState` (`self.State`)))
  (switch `/Game/VIDAEnfermagem/Core/E_ProcedureState` _output_get
    (:`NewEnumerator3`
      (set `self.State` "NewEnumerator2"))))

(event `SyringeMounted`
  (set `self.bSyringeMounted` true)
  (bind _output_get (set `self.PreviousState` (`self.State`)))
  (switch `/Game/VIDAEnfermagem/Core/E_ProcedureState` _output_get
    (:`NewEnumerator4`
      (set `self.State` "NewEnumerator5"))))

(event `PatientPunctured`
  (if (not (and (`self.bPatientSterilyzed`) (`self.bHandsWashed`)))
    (switch `/Game/VIDAEnfermagem/Core/E_ProcedureState` (`self.State`)
      (:`NewEnumerator0`
        _)
      (:`NewEnumerator1`
        _)
      (:`NewEnumerator3`
        _)
      (:`NewEnumerator2`
        _)
      (:`NewEnumerator4`
        _))
    (`/Game/VIDAEnfermagem/Core/BP_ScoreHandler.Serious fault` (`self.ScoreHandler`))))

(event `VeinPunctured`
  (bind _output_get (set `self.PreviousState` (`self.State`)))
  (switch `/Game/VIDAEnfermagem/Core/E_ProcedureState` _output_get
    (:`NewEnumerator5`
      (set `self.State` "NewEnumerator6"))))

(event `VeinDepunctured`
  (bind _output_get (set `self.PreviousState` (`self.State`)))
  (switch `/Game/VIDAEnfermagem/Core/E_ProcedureState` _output_get
    (:`NewEnumerator6`
      (set `self.State` "NewEnumerator5"))))

(event `BloodCollectinStarted`
  ;[1 1 1] "Debouncing
  (if (not (`self.bCollectionStarted`))
    (set `self.bCollectionStarted` true)
    (if (not (`self.bGlassesPutOn`))
      (`/Game/VIDAEnfermagem/Core/BP_ScoreHandler.Weak Fault` (`self.ScoreHandler`)))
    (if (not (`self.bPatientBuckled`))
      (`/Game/VIDAEnfermagem/Core/BP_ScoreHandler.Medium Fault` (`self.ScoreHandler`)))
    (bind _output_get (set `self.PreviousState` (`self.State`)))
    (switch `/Game/VIDAEnfermagem/Core/E_ProcedureState` _output_get
      (:`NewEnumerator6`
        (set `self.State` "NewEnumerator11")))))

(event `Patient Unbuckled`
  (set `self.bPatientBuckled` false)
  (bind _output_get (set `self.PreviousState` (`self.State`)))
  (switch `/Game/VIDAEnfermagem/Core/E_ProcedureState` _output_get
    (:`NewEnumerator2`
      (`/Game/VIDAEnfermagem/Core/BP_ScoreHandler.Weak Fault` (`self.ScoreHandler`) :!label _label)
      (set `self.State` "NewEnumerator3"))
    (:`NewEnumerator4`
      (goto _label))
    (:`NewEnumerator5`
      (goto _label))
    (:`NewEnumerator11`
      (set `self.State` "NewEnumerator12"))))

(event `BloodCollected`
  (set `self.bBloodCollected` true)
  (bind _output_get (set `self.PreviousState` (`self.State`)))
  (switch `/Game/VIDAEnfermagem/Core/E_ProcedureState` _output_get
    (:`NewEnumerator2`
      (`/Game/VIDAEnfermagem/Core/BP_ScoreHandler.Weak Fault` (`self.ScoreHandler`)))
    (:`NewEnumerator12`
      (set `self.State` "NewEnumerator7"))))

(event `SampleHomogenized`
  (bind _output_get (set `self.PreviousState` (`self.State`)))
  (switch `/Game/VIDAEnfermagem/Core/E_ProcedureState` _output_get
    (:`NewEnumerator7`
      (if (`self.bProcedureFinished`)
        (set `self.State` "NewEnumerator8")
        (else
          (set `self.State` "NewEnumerator9"))))))

(event `PatientDepunctured`
  (if (`self.bBloodCollected`)
    (set `self.bProcedureFinished` true)
    (bind _output_get (set `self.PreviousState` (`self.State`)))
    (switch `/Game/VIDAEnfermagem/Core/E_ProcedureState` _output_get
      (:`NewEnumerator5`
        (`/Game/VIDAEnfermagem/Core/BP_ScoreHandler.Weak Fault` (`self.ScoreHandler`) :!label _label_2))
      (:`NewEnumerator7`
        (goto _label_2))
      (:`NewEnumerator9`
        (set `self.State` "NewEnumerator8")))))

(event `Failure`
  (set `self.State` "NewEnumerator10"))

(fn `UserConstructionScript`)