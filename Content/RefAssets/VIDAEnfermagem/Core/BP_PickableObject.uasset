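; BP_PickableObject is an object the player's BP_FloatingHands pawn can hold in either hand, apparently a base class with an empty SetReferences hook.
; It saves its relative root transform at BeginPlay and exposes it through getters, alongside per-hand transforms, a pickup-enabled flag and an immediate-release flag.
; A shared macro finds the holding hand by comparing display names with the pawn's attached objects, driving DetachFromHand and IsAttachedToRight.
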(event `self.ReceiveBeginPlay`
  (set `self.transformPadrao` (`SceneComponent.GetRelativeTransform` (`self.DefaultSceneRoot`)))
  (`self.SetReferences`))

(event `self.ReceiveTick`
  (params (DeltaSeconds :type "Float (single-precision)")))

(fn `DetachFromHand`
  (bind _asbp_floating_hands (cast `/Game/VIDAEnfermagem/Characters/Player/BP_FloatingHands` (`GameplayStatics.GetPlayerPawn` 0)))
  (`self.MãoDireitaOuEsquerda`
    (:`Direita`
      (`/Game/VIDAEnfermagem/Characters/Player/BP_FloatingHands.Soltar_D` _asbp_floating_hands))
    (:`Esquerda`
      (`/Game/VIDAEnfermagem/Characters/Player/BP_FloatingHands.Soltar_E` _asbp_floating_hands))))

(fn `GetDefaultTransform`
  (returns (transformPadrao :type "Transform Structure"))
  (return (`self.transformPadrao`)))

(fn `GetLeftHandTransform`
  (returns (transformMaoEsquerda :type "Transform Structure"))
  (return (`self.transformMaoEsquerda`)))

(fn `GetRightHandTransform`
  (returns (transformMaoDireita :type "Transform Structure"))
  (return (`self.transformMaoDireita`)))

(fn `getSoltarImediatamente`
  (returns (soltarImediatamente :type Boolean))
  (return (`self.triggerBandeja`)))

(fn `IsAttachedToRight`
  (returns (NewParam :type Boolean))
  (`self.MãoDireitaOuEsquerda`
    (:`Direita`
      (return true))
    (:`Esquerda`
      (return false))))

(fn `IsPickingEnabled`
  (returns (pegarAtivado :type Boolean))
  (return (`self.pegarAtivado`)))

(fn `SetReferences`)

(fn `UserConstructionScript`)