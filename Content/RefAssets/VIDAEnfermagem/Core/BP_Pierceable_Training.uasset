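; BP_Pierceable_Training is a training target whose sphere visually signals the piercing step of a training sequence.
; BeginPlay gives the sphere a dynamic material instance.
; Tick polls the TrainingFSM state: Perforating turns the sphere green and plays a timeline driving a brightness glow, while End restores light gray and stops the glow.
; DoOnce nodes make each state change fire only once despite the per-frame check.
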(event `self.ReceiveBeginPlay`
  (bind _returnvalue (`KismetMaterialLibrary.CreateDynamicMaterialInstance` "/Game/VIDAEnfermagem/MaterialLibrary/SimpleColors/M_LightGray.M_LightGray"))
  (bind _output_get (set `self.Dynamic Material` _returnvalue))
  (`PrimitiveComponent.SetMaterial` (`self.Sphere`) 0 _output_get))

(event `self.ReceiveTick`
  (params (DeltaSeconds :type "Float (single-precision)"))
  (bind _dynamic_material (`self.Dynamic Material`))
  (switch `/Game/VIDAEnfermagem/Core/E_TrainingState` (`/Game/VIDAEnfermagem/Core/BP_TrainingFSM.State` (`self.TrainingFSM`))
    (:`NewEnumerator4`
      (`/Engine/EditorBlueprintResources/StandardMacros.DoOnce` false
        (:`Completed`
          (`MaterialInstanceDynamic.SetVectorParameterValue` _dynamic_material "color" (struct :`R` 0.074769 :`G` 1.0 :`A` 1.0))
          (bind (_direction _glow) (`Timeline|Timeline_0` :!via `PlayFromStart` :!label _label)
            (:`Update`
              (`MaterialInstanceDynamic.SetScalarParameterValue` (`self.Dynamic Material`) "Brightness" _glow))))))
    (:`NewEnumerator7`
      (`/Engine/EditorBlueprintResources/StandardMacros.DoOnce` false
        (:`Completed`
          (`MaterialInstanceDynamic.SetVectorParameterValue` _dynamic_material "color" (struct :`R` 0.8 :`G` 0.8 :`B` 0.8 :`A` 1.0))
          (`|ExecutionSequence`
            (:`then_0`
              (goto _label :!via `Stop`))
            (:`then_1`
              (`MaterialInstanceDynamic.SetScalarParameterValue` (`self.Dynamic Material`) "Brightness" 0.0))))))))

(fn `UserConstructionScript`)