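; State machine that sequences a training tutorial from welcome through look-around, movement, cube and syringe pickup, to perforation and end.
; TelevisionLookedAt drives the early steps on timed delays, toggling the floating-hands character's Trace flag, while pickup and perforation events drive the later ones.
; ObjectPerforated is handled only in PickingSyringe, not Perforating.
; The N key skips forward one state, and Tick prints the current state for debugging.
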(event `self.ReceiveTick`
  (params (DeltaSeconds :type "Float (single-precision)"))
  (`KismetSystemLibrary.PrintString` (`|GetEnumeratorNameAsString` (`self.State`)) true true (struct :`G` 0.66 :`B` 1.0 :`A` 1.0) DeltaSeconds))

(event `self.ReceiveBeginPlay`
  (set `self.State` "NewEnumerator8")
  (bind _asbp_floating_hands_training (cast `/Game/VIDAEnfermagem/Characters/Player/BP_FloatingHands_Training` (`GameplayStatics.GetPlayerCharacter` 0)))
  (set `/Game/VIDAEnfermagem/Characters/Player/BP_FloatingHands_Training.bTrace` true _asbp_floating_hands_training))

(event `TelevisionLookedAt`
  (switch `/Game/VIDAEnfermagem/Core/E_TrainingState` (`self.State`)
    (:`NewEnumerator8`
      (`KismetSystemLibrary.Delay` 3.0)
      (set `self.State` "NewEnumerator9"))
    (:`NewEnumerator9`
      (`KismetSystemLibrary.Delay` 5.0)
      (set `self.State` "NewEnumerator0")
      (bind _asbp_floating_hands_training (cast `/Game/VIDAEnfermagem/Characters/Player/BP_FloatingHands_Training` (`GameplayStatics.GetPlayerCharacter` 0)))
      (set `/Game/VIDAEnfermagem/Characters/Player/BP_FloatingHands_Training.bTrace` false _asbp_floating_hands_training)
      (`KismetSystemLibrary.Delay` 10.0)
      (set `/Game/VIDAEnfermagem/Characters/Player/BP_FloatingHands_Training.bTrace` true _asbp_floating_hands_training))
    (:`NewEnumerator0`
      (`KismetSystemLibrary.Delay` 3.0)
      (set `self.State` "NewEnumerator1")
      (bind _asbp_floating_hands_training_2 (cast `/Game/VIDAEnfermagem/Characters/Player/BP_FloatingHands_Training` (`GameplayStatics.GetPlayerCharacter` 0)))
      (set `/Game/VIDAEnfermagem/Characters/Player/BP_FloatingHands_Training.bTrace` false _asbp_floating_hands_training_2)
      (`KismetSystemLibrary.Delay` 10.0)
      (set `/Game/VIDAEnfermagem/Characters/Player/BP_FloatingHands_Training.bTrace` true _asbp_floating_hands_training_2))
    (:`NewEnumerator1`
      (bind _asbp_floating_hands_training_3 (cast `/Game/VIDAEnfermagem/Characters/Player/BP_FloatingHands_Training` (`GameplayStatics.GetPlayerCharacter` 0)))
      (set `/Game/VIDAEnfermagem/Characters/Player/BP_FloatingHands_Training.bTrace` false _asbp_floating_hands_training_3)
      (`KismetSystemLibrary.Delay` 3.0)
      (set `self.State` "NewEnumerator10")
      (`KismetSystemLibrary.Delay` 8.0)
      (set `self.State` "NewEnumerator2"))))

(event `CubePicked`
  (switch `/Game/VIDAEnfermagem/Core/E_TrainingState` (`self.State`)
    (:`NewEnumerator2`
      (set `self.State` "NewEnumerator3"))))

(event `Key|N` :consume false :overrideparent false
  (params (Key :type "Key Structure"))
  (:`Pressed`
    (switch `/Game/VIDAEnfermagem/Core/E_TrainingState` (`self.State`)
      (:`NewEnumerator8`
        (set `self.State` "NewEnumerator9"))
      (:`NewEnumerator9`
        (set `self.State` "NewEnumerator0"))
      (:`NewEnumerator0`
        (set `self.State` "NewEnumerator1"))
      (:`NewEnumerator1`
        (set `self.State` "NewEnumerator10"))
      (:`NewEnumerator10`
        (set `self.State` "NewEnumerator2"))
      (:`NewEnumerator2`
        (set `self.State` "NewEnumerator3"))
      (:`NewEnumerator3`
        (set `self.State` "NewEnumerator4"))
      (:`NewEnumerator4`
        (set `self.State` "NewEnumerator7")))))

(event `SyringePicked`
  (switch `/Game/VIDAEnfermagem/Core/E_TrainingState` (`self.State`)
    (:`NewEnumerator3`
      (set `self.State` "NewEnumerator4"))))

(event `ObjectPerforated`
  (switch `/Game/VIDAEnfermagem/Core/E_TrainingState` (`self.State`)
    (:`NewEnumerator3`
      (set `self.State` "NewEnumerator7")
      (bind _asbp_floating_hands_training (cast `/Game/VIDAEnfermagem/Characters/Player/BP_FloatingHands_Training` (`GameplayStatics.GetPlayerCharacter` 0)))
      (set `/Game/VIDAEnfermagem/Characters/Player/BP_FloatingHands_Training.bTrace` true _asbp_floating_hands_training)
      (set `/Game/VIDAEnfermagem/Characters/Player/BP_FloatingHands_Training.DrawTrace` "ForOneFrame" _asbp_floating_hands_training))))

(fn `UserConstructionScript`)