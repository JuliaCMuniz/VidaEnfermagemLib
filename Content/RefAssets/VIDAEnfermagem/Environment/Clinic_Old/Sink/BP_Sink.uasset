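; Clinic sink actor that tracks hand washing by the player's Leap Motion hands.
; Each hand component overlapping the wash trigger starts its own three-second timer, cleared if it leaves early, that marks that hand as sanitized.
; When a hand exits and both are sanitized, it flags completion once, prints a message and writes a hand-hygiene entry to the report.
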(event `self.TriggerLavarMãos.OnComponentBeginOverlap`
  (params (OverlappedComponent :type "PrimitiveComponent Object Reference") (OtherActor :type "Actor Object Reference") (OtherComp :type "PrimitiveComponent Object Reference") (OtherBodyIndex :type Integer) (bFromSweep :type Boolean) (SweepResult :type "HitResult Structure (by ref)"))
  (bind _asbp_custom_leap_low_poly_hand (cast `/Game/VIDAEnfermagem/Core/Leap/BP_CustomLeapLowPolyHand` OtherActor))
  (`|ExecutionSequence`
    (:`then_0`
      (if (and (== (`/Game/VIDAEnfermagem/Core/Leap/BP_CustomLeapLowPolyHand.Right` _asbp_custom_leap_low_poly_hand) OtherComp) (not (`self.Direita Higienizada`)))
        (`KismetSystemLibrary.K2_SetTimer` self "HigienizarMãoDireita" 3.0)))
    (:`then_1`
      (if (and (== (`/Game/VIDAEnfermagem/Core/Leap/BP_CustomLeapLowPolyHand.Left` _asbp_custom_leap_low_poly_hand) OtherComp) (not (`self.Esquerda Higienizada`)))
        (`KismetSystemLibrary.K2_SetTimer` self "HigienizarMãoEsquerda" 3.0)))))

(event `self.TriggerLavarMãos.OnComponentEndOverlap`
  (params (OverlappedComponent :type "PrimitiveComponent Object Reference") (OtherActor :type "Actor Object Reference") (OtherComp :type "PrimitiveComponent Object Reference") (OtherBodyIndex :type Integer))
  (bind _asbp_custom_leap_low_poly_hand (cast `/Game/VIDAEnfermagem/Core/Leap/BP_CustomLeapLowPolyHand` OtherActor))
  (`|ExecutionSequence`
    (:`then_0`
      (if (== (`/Game/VIDAEnfermagem/Core/Leap/BP_CustomLeapLowPolyHand.Right` _asbp_custom_leap_low_poly_hand) OtherComp)
        (`KismetSystemLibrary.K2_ClearTimer` self "HigienizarMãoDireita")
        (if (and (`self.Direita Higienizada`) (`self.Esquerda Higienizada`) (not (`self.Mãos Higienizadas`))) :!label _label
          (set `self.Mãos Higienizadas` true)
          (`KismetSystemLibrary.PrintString` "Higienização completa!")
          (`/Game/VIDAEnfermagem/Core/WriteText.EscreveRelatorio` "Higienizou mãos"))))
    (:`then_1`
      (if (== (`/Game/VIDAEnfermagem/Core/Leap/BP_CustomLeapLowPolyHand.Left` _asbp_custom_leap_low_poly_hand) OtherComp)
        (`KismetSystemLibrary.K2_ClearTimer` self "HigienizarMãoEsquerda")
        (goto _label)))))

(fn `HigienizarMãoDireita`
  (set `self.Direita Higienizada` true)
  (`KismetSystemLibrary.PrintString` "Direita Higienizada!"))

(fn `HigienizarMãoEsquerda`
  (set `self.Esquerda Higienizada` true)
  (`KismetSystemLibrary.PrintString` "Esquerda Higienizada!"))

(fn `UserConstructionScript`)