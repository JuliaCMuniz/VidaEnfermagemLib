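; Clinic television actor with an LED mesh and a widget that it shows in the Treinamento and Procedimento levels.
; On BeginPlay it gives the LED a dynamic M_LED material instance, then switches on the current level name to make the widget visible.
; Unconnected leftover nodes would set the material's On parameter to zero or show the widget based on the GameInstance's GuidedMode setting, but never run.
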(event `self.ReceiveBeginPlay`
  (bind _returnvalue (`KismetMaterialLibrary.CreateDynamicMaterialInstance` "/Game/VIDAEnfermagem/Environment/Clinic/Television/M_LED.M_LED"))
  (bind _output_get (set `self.NewVar_0` _returnvalue))
  (`PrimitiveComponent.SetMaterial` (`self.Led`) 0 _output_get)
  (bind _returnvalue_2 (`GameplayStatics.GetCurrentLevelName` true))
  (switch `string` _returnvalue_2
    (:`Treinamento`
      _)
    (:`Procedimento`
      _))
  (`SceneComponent.SetVisibility` (`self.Widget`) true false))

(fn `UserConstructionScript`)