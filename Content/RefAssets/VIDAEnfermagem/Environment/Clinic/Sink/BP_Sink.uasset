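; BP_Sink is a clinic sink where the VR player washes both hands.
; When a VRPawnCustom overlaps it, water particles and sound start, then stop when the overlap ends.
; On overlap begin, it reads LeftHand or RightHand tags from the third parent of each overlapping component to mark that hand washed.
; Once both flags are set it calls the OnBothHandsWashed dispatcher, and no graph here resets them.
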(event `self.ReceiveActorBeginOverlap`
  (params (OtherActor :type "Actor Object Reference"))
  (if (== (`GameplayStatics.GetObjectClass` OtherActor) "/Game/Blueprints/VRPawn/VRPawnCustom.VRPawnCustom_C")
    (`self.ShowWater`)
    (for _array_element (`self.GetOverlappingComponents`)
      (bind _parents (`SceneComponent.GetParentComponents` _array_element))
      (if (`KismetArrayLibrary.Array_IsValidIndex` _parents 2)
        (for _array_element_2 (`ActorComponent.ComponentTags` (`|GetArrayItem` _parents 2))
          (if (== _array_element_2 "LeftHand")
            (`self.WashLeftHand`)
            (elif (== _array_element_2 "RightHand")
              (`self.WashRightHand`))))))))

(event `self.ReceiveActorEndOverlap`
  (params (OtherActor :type "Actor Object Reference"))
  (if (== (`GameplayStatics.GetObjectClass` OtherActor) "/Game/Blueprints/VRPawn/VRPawnCustom.VRPawnCustom_C")
    (`self.EndWater`)))

(fn `EndWater`
  (`AudioComponent.FadeOut` (`self.aguasom`) 1.0 0.0 "Linear")
  (`ActorComponent.Deactivate` (`self.WaterParticleSystem`)))

(fn `ShowWater`
  (`AudioComponent.FadeIn` (`self.aguasom`) 1.0 1.0 0.0 "Linear")
  (`ActorComponent.Activate` (`self.WaterParticleSystem`) false))

(fn `UserConstructionScript`)

(fn `WashLeftHand`
  (set `self.LeftWashed` true)
  (if (`self.RightWashed`)
    (`self.OnBothHandsWashed`)))

(fn `WashRightHand`
  (set `self.RightWashed` true)
  (if (`self.LeftWashed`)
    (`self.OnBothHandsWashed`)))