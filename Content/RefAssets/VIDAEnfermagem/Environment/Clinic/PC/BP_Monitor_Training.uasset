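; BP_Monitor_Training is a clinic PC monitor that lights up and shows text when the training session ends.
; BeginPlay creates a dynamic material instance for the monitor mesh.
; Tick polls the TrainingFSM state and, on End, uses a DoOnce to reveal the TextRender and start a timeline that drives the material's Brightness.
; An unconnected branch that would stop the glow and zero Brightness never runs.
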(event `self.ReceiveBeginPlay`
  (bind _returnvalue (`KismetMaterialLibrary.CreateDynamicMaterialInstance` "/Game/VIDAEnfermagem/Environment/Clinic/PC/10120_LCD_Computer_Monitor_v01.10120_LCD_Computer_Monitor_v01"))
  (bind _output_get (set `self.DynamicMaterial` _returnvalue))
  (`PrimitiveComponent.SetMaterial` (`self.Monitor`) 0 _output_get))

(event `self.ReceiveTick`
  (params (DeltaSeconds :type "Float (single-precision)"))
  (switch `/Game/VIDAEnfermagem/Core/E_TrainingState` (`/Game/VIDAEnfermagem/Core/BP_TrainingFSM.State` (`self.TrainingFSM`))
    (:`NewEnumerator7`
      (`/Engine/EditorBlueprintResources/StandardMacros.DoOnce` false
        (:`Completed`
          (`SceneComponent.SetVisibility` (`self.TextRender`) true false)
          (bind (_direction _glow) (`Timeline|Timeline_0` :!via `PlayFromStart`)
            (:`Update`
              (`MaterialInstanceDynamic.SetScalarParameterValue` (`self.DynamicMaterial`) "Brightness" _glow))))))))

(fn `UserConstructionScript`)