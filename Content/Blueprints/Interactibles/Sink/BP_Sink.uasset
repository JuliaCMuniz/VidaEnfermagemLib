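; Interactive VR sink that detects when the player has washed both hands.
; Actor overlap with VRPawnCustom starts and stops the water particles and fades the water sound in and out.
; WashingTrigger identifies each hand by the first tag on the overlapping component's third parent, setting its washed flag.
; Once both flags are set, it calls the OnBothHandsWashed dispatcher; BeginSink clears both flags.
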(event `self.ReceiveActorBeginOverlap`
  (params (OtherActor :type "Actor Object Reference"))
  (if (== (`GameplayStatics.GetObjectClass` OtherActor) "/Game/Blueprints/VRPawn/VRPawnCustom.VRPawnCustom_C")
    (`self.ShowWater`)))

(event `self.ReceiveActorEndOverlap`
  (params (OtherActor :type "Actor Object Reference"))
  (if (== (`GameplayStatics.GetObjectClass` OtherActor) "/Game/Blueprints/VRPawn/VRPawnCustom.VRPawnCustom_C")
    (`self.EndWater`)))

(event `self.WashingTrigger.OnComponentBeginOverlap`
  (params (OverlappedComponent :type "PrimitiveComponent Object Reference") (OtherActor :type "Actor Object Reference") (OtherComp :type "PrimitiveComponent Object Reference") (OtherBodyIndex :type Integer) (bFromSweep :type Boolean) (SweepResult :type "HitResult Structure (by ref)"))
  (bind _parents (`SceneComponent.GetParentComponents` OtherComp))
  (bind _output (`|GetArrayItem` (`ActorComponent.ComponentTags` (`|GetArrayItem` _parents 2))))
  (if (`KismetArrayLibrary.Array_IsValidIndex` _parents 2)
    (if (== _output "LeftHand")
      (`self.WashLeftHand`)
      (elif (== _output "RightHand")
        (`self.WashRightHand`)))))

(event `Event BeginSink`
  (set `self.RightWashed` false)
  (set `self.LeftWashed` false))

(fn `EndWater`
  (`AudioComponent.FadeOut` (`self.aguasom`) 1.0 0.0 "Linear")
  (`ActorComponent.Deactivate` (`self.WaterParticleSystem`)))

(fn `ShowWater`
  (`AudioComponent.FadeIn` (`self.aguasom`) 1.0 1.0 0.0 "Linear")
  (`ActorComponent.Activate` (`self.WaterParticleSystem`) false))

(fn `UserConstructionScript`)

(fn `WashLeftHand`
  (set `self.LeftWashed` true)
  (if (`self.RightWashed`)
    (`self.OnBothHandsWashed`)))

(fn `WashRightHand`
  (set `self.RightWashed` true)
  (if (`self.LeftWashed`)
    (`self.OnBothHandsWashed`)))