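; BP_BaseGrabbable is a base Blueprint for objects grabbed through the ISDK (Isdk) interaction components.
; On BeginPlay it registers InteractibleStaticMesh as the IsdkGrabbableInteractable's collider and links that interactable to the IsdkGrabbable component.
; It then constructs a free transformer at runtime for single grabs and sets the mesh as the transform target, so grabs move the mesh.
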(event `self.ReceiveBeginPlay`
  (`|ExecutionSequence`
    (:`then_0`
      ;[1 1 1] Set Collider and Grabbable
      (`IsdkGrabbableComponent.SetCollider` (`self.IsdkGrabbableInteractable`) (`self.InteractibleStaticMesh`))
      (set `IsdkGrabbableComponent.Grabbable` (`self.IsdkGrabbable`) (`self.IsdkGrabbableInteractable`)))
    (:`then_1`
      ;[1 1 1] Link Transform
      (bind _returnvalue (`|GenericCreateObject` "/Script/OculusInteraction.IsdkGrabFreeTransformer"))
      (set `IsdkGrabbable.SingleGrabTransformer` _returnvalue (`self.IsdkGrabbable`))
      (set `IsdkGrabbable.TransformTarget` (`self.InteractibleStaticMesh`) (`self.IsdkGrabbable`)))))

(fn `UserConstructionScript`)