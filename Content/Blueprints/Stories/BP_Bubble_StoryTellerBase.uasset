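; Base storyteller actor that plays StoryList in order, gating each story behind an action bubble.
; It spawns up to three BP_ActionBubbles at tagged anchors for the current and upcoming stories, marking the first as right.
; Destroying that bubble clears the rest and spawns the story actor with its steps, or directly if none exist.
; Each finished story advances the index and respawns bubbles; the last fires OnStoryTellerEnded.
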(event `self.ReceiveBeginPlay`
  (if (> (`KismetArrayLibrary.Array_Length` (`self.StoryList`)) 0)
    (set `self.CurrentStoryIndex` 0)
    (`self.SpawnBubbles`)
    (`self.Event BubblePrep`)))

(event `Event BubblePrep`
  (bind _activebubbles (`self.ActiveBubbles`))
  (bind _output (`|GetArrayItem` _activebubbles))
  (if (> (`KismetArrayLibrary.Array_Length` _activebubbles) 0)
    (add `/Game/Blueprints/Stories/UI/BP_ActionBubble.OnBubbleDestroyed` _output (delegate `Event BubblePop`))
    (`/Game/Blueprints/Stories/UI/BP_ActionBubble.SetBubbleRight` _output)
    (else
      (`self.StartStory` (`self.CurrentStoryIndex`) :!label _label))))

(event `Event BubblePop`
  (`self.CleanBubbleArray`)
  (goto _label))

(event `Event StoryFinished`
  (bind _currentstoryindex (`self.CurrentStoryIndex`))
  (bind _storylist (`self.StoryList`))
  (bind _returnvalue (+ _currentstoryindex 1))
  (if (== (`KismetArrayLibrary.Array_LastIndex` _storylist) _currentstoryindex)
    ;[1 1 1] LAST STORY
    (`self.OnStoryTellerEnded`)
    (elif (`KismetArrayLibrary.Array_IsValidIndex` _storylist _returnvalue)
      (set `self.CurrentStoryIndex` _returnvalue)
      (`self.SpawnBubbles`)
      (`self.Event BubblePrep`))))

(fn `CleanBubbleArray`
  (locals (CleanArray :type "Array of /Game/Blueprints/Stories/UI/BP_ActionBubble Object Reference"))
  (bind _activebubbles (`self.ActiveBubbles`))
  (for _array_element _activebubbles
    (`/Engine/EditorBlueprintResources/StandardMacros.IsValid` _array_element
      (:`Is Valid`
        (`self.K2_DestroyActor` _array_element))))
  (`KismetArrayLibrary.Array_Clear` _activebubbles)
  (return))

(fn `SpawnBubbles`
  (bind _storylist (`self.StoryList`))
  (bind _returnvalue (`KismetArrayLibrary.Array_Length` (`self.ActiveBubbles`)))
  (bind _returnvalue_2 (+ _returnvalue (`self.CurrentStoryIndex`)))
  (while (< _returnvalue 3)
    (if (`KismetArrayLibrary.Array_IsValidIndex` _storylist _returnvalue_2)
      (bind _outactors (`GameplayStatics.GetAllActorsWithTag` (`.StoryAnchorTag_26_B840F19A422252649D125284DA93EE8B` (break `/Game/Blueprints/Stories/BubbleStory` (`|GetArrayItem` _storylist _returnvalue_2)))))
      (bind _output (`|GetArrayItem` _outactors))
      (if (`KismetSystemLibrary.IsValid` _output)
        (bind _returnvalue_3 (`|SpawnActorFromClass` "/Game/Blueprints/Stories/UI/BP_ActionBubble.BP_ActionBubble_C" (`self.GetTransform` _output) "Undefined" "MultiplyWithRoot" null null))
        (`KismetArrayLibrary.Array_Add` (`self.ActiveBubbles`) _returnvalue_3))
      (else
        (return))))
  (return))

(fn `StartStory`
  (params (StoryIndex :type Integer))
  (bind _currentstoryobject (`self.CurrentStoryObject`))
  (bind (_story _storyanchortag _storysteps) (break `/Game/Blueprints/Stories/BubbleStory` (`|GetArrayItem` (`self.StoryList`) StoryIndex)))
  (if (`KismetSystemLibrary.IsValid` _currentstoryobject)
    (remove `/Game/Blueprints/Stories/BP_Bubble_StoryBase.OnStoryFinished` _currentstoryobject (`|CreateDelegate` :!event `Event StoryFinished`))
    (`self.K2_DestroyActor` _currentstoryobject))
  (`|ExecutionSequence`
    (:`then_0`
      (bind _returnvalue (`|SpawnActorFromClass` _story (`self.GetTransform`) "Undefined" "MultiplyWithRoot" null _storysteps null))
      (bind _output_get (set `self.CurrentStoryObject` _returnvalue)))
    (:`then_1`
      (add `/Game/Blueprints/Stories/BP_Bubble_StoryBase.OnStoryFinished` (`self.CurrentStoryObject`) (`|CreateDelegate` :!event `Event StoryFinished`)))))

(fn `UserConstructionScript`)