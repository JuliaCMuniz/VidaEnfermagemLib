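; Base story Blueprint that tracks progress through an ordered list of steps and signals when the story finishes.
; BeginPlay takes the first step and binds to its step-ended event, or prints a warning if the list is empty.
; Each ended step is unbound, then UpdateStep calls OnStoryFinished after the last one.
; Its branch for advancing to the next step uses a reversed length comparison, so valid intermediate steps never advance.
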(event `self.ReceiveBeginPlay`
  ;[1 1 1] Check if there are steps
  (if (> (`KismetArrayLibrary.Array_Length` (`self.StepList`)) 0)
    (bind _output_get (set `self.CurrentStep` (`|GetArrayItem` (`self.StepList`))))
    (add `/Game/Blueprints/Stories/BP_StepBase.OnStepEnded` (`|ConvertAsset` _output_get) (delegate `OnStepFinished`))
    (else
      (`KismetSystemLibrary.PrintText` "Missing StepList"))))

(event `OnStepFinished`
  (remove `/Game/Blueprints/Stories/BP_StepBase.OnStepEnded` (`|ConvertAsset` (`self.CurrentStep`)) (delegate `OnStepFinished`))
  (bind _stepresolved (`self.UpdateStep`))
  (add `/Game/Blueprints/Stories/BP_StepBase.OnStepEnded` _stepresolved (delegate `OnStepFinished`)))

(fn `UpdateStep`
  (returns (StepResolved :type "/Game/Blueprints/Stories/BP_StepBase Object Reference"))
  (bind _steplist (`self.StepList`))
  (bind _returnvalue (`KismetArrayLibrary.Array_Length` _steplist))
  (bind _returnvalue_2 (+ (`KismetArrayLibrary.Array_Find` _steplist (`self.CurrentStep`)) 1))
  (if (== _returnvalue _returnvalue_2)
    (`self.OnStoryFinished`)
    (elif (< _returnvalue _returnvalue_2)
      (bind _output_get (set `self.CurrentStep` (`|GetArrayItem` _steplist _returnvalue_2)))
      (return (`|ConvertAsset` _output_get)))))

(fn `UserConstructionScript`)