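; BP_Dialogue_Step is a story step that runs a quiz-style dialogue and signals step completion when the answers end.
; On BeginPlay it finds the interactable widget tagged DialogueWidget, makes it visible, binds to its BP_Quiz events and shows the question.
; Wrong answers pass their explanation to the BP_ErrorMessage widget on the ErrorWidget-tagged actor, while correct answers have an empty handler.
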(event `self.ReceiveBeginPlay`
  (bind _outactors (`GameplayStatics.GetAllActorsWithTag` "DialogueWidget"))
  (bind _asisdk_interactable_widget (cast `IsdkInteractableWidget` (`|GetArrayItem` _outactors)))
  (bind _interactablewidgetcomponent (`IsdkInteractableWidget.InteractableWidgetComponent` _asisdk_interactable_widget))
  (`SceneComponent.SetVisibility` _interactablewidgetcomponent true true)
  (bind _asbp_quiz (cast `/Game/Blueprints/Interface/BP_Quiz` (`WidgetComponent.GetWidget` (`IsdkInteractableWidgetComponent.Widget` _interactablewidgetcomponent))))
  (add `/Game/Blueprints/Interface/BP_Quiz.OnWrongAnswerSelected` _asbp_quiz (delegate `CustomEvent_1`))
  (add `/Game/Blueprints/Interface/BP_Quiz.OnCorrectAnswerSelected` _asbp_quiz (delegate `CustomEvent_0`))
  (add `/Game/Blueprints/Interface/BP_Quiz.OnAnswersEnded` _asbp_quiz (delegate `Event AnswersEnded`))
  (`/Game/Blueprints/Interface/BP_Quiz.ShowQuestion` _asbp_quiz))

(event `CustomEvent_1`
  (params (ExplanationMessage :type String))
  (`self.TreatWrongAnswer` ExplanationMessage))

(event `CustomEvent_0`)

(event `Event AnswersEnded`
  (`self.OnStepFinished`))

(fn `TreatWrongAnswer`
  (params (ExplanationMessage :type String))
  (bind _outactors (`GameplayStatics.GetAllActorsWithTag` "ErrorWidget"))
  (bind _asisdk_interactable_widget (cast `IsdkInteractableWidget` (`|GetArrayItem` _outactors)))
  (bind _asbp_error_message (cast `/Game/Blueprints/Interface/BP_ErrorMessage` (`WidgetComponent.GetWidget` (`IsdkInteractableWidgetComponent.Widget` (`IsdkInteractableWidget.InteractableWidgetComponent` _asisdk_interactable_widget)))))
  (`/Game/Blueprints/Interface/BP_ErrorMessage.SetTextMessage` _asbp_error_message ExplanationMessage))

(fn `UserConstructionScript`
  (`parent.UserConstructionScript`))