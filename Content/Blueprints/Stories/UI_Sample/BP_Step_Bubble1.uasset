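; BP_Step_Bubble1 is a story step in the UI sample that presents an action bubble to be triggered with the right hand.
; On BeginPlay it spawns a BP_ActionBubble at its own transform and binds to its left and right hand trigger events.
; A left-hand trigger shows the bubble's warning message, while a right-hand trigger shows the success message and calls OnStepFinished to signal completion.
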(event `self.ReceiveBeginPlay`
  (`KismetSystemLibrary.PrintString` "Starting Bubble 1")
  (bind _returnvalue (`|SpawnActorFromClass` "/Game/Blueprints/Stories/UI/BP_ActionBubble.BP_ActionBubble_C" (`self.GetTransform`) "Undefined" "MultiplyWithRoot" null null))
  (bind _output_get (set `self.BubbleObject` _returnvalue))
  (add `/Game/Blueprints/Stories/UI/BP_ActionBubble.OnLeftHandTrigger` _output_get (delegate `Event LeftHandOverlapp`))
  (add `/Game/Blueprints/Stories/UI/BP_ActionBubble.OnRightHandTrigger` _output_get (delegate `Event RightHandOverlapp`)))

(event `Event LeftHandOverlapp`
  (message `/Game/Blueprints/Stories/UI/BubbleUpdateInterface.SetBubbleWarning` (`self.BubbleObject`)))

(event `Event RightHandOverlapp`
  (message `/Game/Blueprints/Stories/UI/BubbleUpdateInterface.SetBubbleSuccess` (`self.BubbleObject`))
  (`KismetSystemLibrary.PrintString` "Finished Bubble 1")
  (`self.OnStepFinished`))

(fn `UserConstructionScript`
  (`parent.UserConstructionScript`))