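; Base story actor that runs an ordered list of steps, each gated by popping an action bubble.
; Bubbles spawn at tagged anchors for up to three steps from the current one, with the first marked as the right one.
; Popping it clears all bubbles and spawns the current step actor.
; Each finished step advances the index and respawns bubbles, while the last fires OnStoryFinished and destroys the story.
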(event `Event BeginStoryRoutine`
  (if (> (`KismetArrayLibrary.Array_Length` (`self.StepList`)) 0)
    (set `self.CurrentStepIndex` 0)
    (`self.SpawnBubbles`)
    (`self.Event BubblePrep`)))

(event `Event BubblePrep`
  (bind _activebubbles (`self.ActiveBubbles`))
  (bind _output (`|GetArrayItem` _activebubbles))
  (if (> (`KismetArrayLibrary.Array_Length` _activebubbles) 0)
    (add `/Game/Blueprints/Stories/UI/BP_ActionBubble.OnBubbleDestroyed` _output (delegate `Event BubblePop`))
    (`/Game/Blueprints/Stories/UI/BP_ActionBubble.SetBubbleRight` _output)
    (else
      (`self.StartStep` (`self.CurrentStepIndex`) :!label _label))))

(event `Event BubblePop`
  (`self.CleanBubbleArray`)
  (goto _label))

(event `Event StepFinished`
  (bind _steplist (`self.StepList`))
  (bind _currentstepindex (`self.CurrentStepIndex`))
  (bind _returnvalue (+ _currentstepindex 1))
  (if (== (`KismetArrayLibrary.Array_LastIndex` _steplist) _currentstepindex)
    ;[1 1 1] LAST STEP
    (`self.OnStoryFinished`)
    (`self.K2_DestroyActor`)
    (elif (`KismetArrayLibrary.Array_IsValidIndex` _steplist _returnvalue)
      (set `self.CurrentStepIndex` _returnvalue)
      (`self.SpawnBubbles`)
      (`self.Event BubblePrep`))))

(fn `CleanBubbleArray`
  (bind _activebubbles (`self.ActiveBubbles`))
  (for _array_element _activebubbles
    (`/Engine/EditorBlueprintResources/StandardMacros.IsValid` _array_element
      (:`Is Valid`
        (`self.K2_DestroyActor` _array_element))))
  (`KismetArrayLibrary.Array_Clear` _activebubbles)
  (return))

(fn `SpawnBubbles`
  (bind _steplist (`self.StepList`))
  (bind _returnvalue (`KismetArrayLibrary.Array_Length` (`self.ActiveBubbles`)))
  (bind _returnvalue_2 (+ _returnvalue (`self.CurrentStepIndex`)))
  (while (< _returnvalue 3)
    (if (`KismetArrayLibrary.Array_IsValidIndex` _steplist _returnvalue_2)
      (bind _outactors (`GameplayStatics.GetAllActorsWithTag` (`.StepAnchorTag_12_6512213B4D7F89C400F241A9D4330C8C` (break `/Game/Blueprints/Stories/BubbleStep` (`|GetArrayItem` _steplist _returnvalue_2)))))
      (bind _output (`|GetArrayItem` _outactors))
      (if (`KismetSystemLibrary.IsValid` _output)
        (bind _returnvalue_3 (`|SpawnActorFromClass` "/Game/Blueprints/Stories/UI/BP_ActionBubble.BP_ActionBubble_C" (`self.GetTransform` _output) "Undefined" "MultiplyWithRoot" null null))
        (`KismetArrayLibrary.Array_Add` (`self.ActiveBubbles`) _returnvalue_3))
      (else
        (return))))
  (return))

(fn `StartStep`
  (params (StoryIndex :type Integer))
  (bind _currentstep (`self.CurrentStep`))
  (if (`KismetSystemLibrary.IsValid` _currentstep)
    (remove `/Game/Blueprints/Stories/BP_StepBase.OnStepFinished` _currentstep (`|CreateDelegate` :!event `Event StepFinished`))
    (`self.K2_DestroyActor` _currentstep))
  (`|ExecutionSequence`
    (:`then_0`
      (bind _returnvalue (`|SpawnActorFromClass` (`.Step_3_AF7FA3004CF6C6459D83D9A27F3C02B4` (break `/Game/Blueprints/Stories/BubbleStep` (`|GetArrayItem` (`self.StepList`) StoryIndex))) (`self.GetTransform`) "Undefined" "MultiplyWithRoot" null null))
      (set `self.CurrentStep` _returnvalue))
    (:`then_1`
      (add `/Game/Blueprints/Stories/BP_StepBase.OnStepFinished` (`self.CurrentStep`) (`|CreateDelegate` :!event `Event StepFinished`)))))

(fn `UserConstructionScript`)