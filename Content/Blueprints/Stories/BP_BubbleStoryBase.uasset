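; Base Blueprint for stories built around an action bubble that reacts to left, right or any hand triggers.
; BubbleSpawn spawns a BP_ActionBubble at the BubbleTransform actor, falling back to its own transform when that is invalid, and binds the bubble's three hand-trigger events.
; Each event forwards to an empty LeftHandTriggered, RightHandTriggered or AnyHandTriggered function, leaving the response to child Blueprints.
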(event `self.ReceiveBeginPlay`
  (`parent.ReceiveBeginPlay`))

(event `Event BubbleSpawn`
  (bind _bubbletransform (`self.BubbleTransform`))
  (if (`KismetSystemLibrary.IsValid` _bubbletransform)
    (bind _bubblereference (`self.SpawnBubble` (`self.GetTransform` _bubbletransform)))
    (add `/Game/Blueprints/Stories/UI/BP_ActionBubble.OnLeftHandTrigger` _bubblereference (delegate `Event OnLeftHandTriggered`))
    (add `/Game/Blueprints/Stories/UI/BP_ActionBubble.OnRightHandTrigger` _bubblereference (delegate `Event OnRightHandTriggered`))
    (add `/Game/Blueprints/Stories/UI/BP_ActionBubble.OnAnyHandTrigger` _bubblereference (delegate `Event OnAnyHandTriggered`))
    (else
      (bind _bubblereference_2 (`self.SpawnBubble` (`self.GetTransform`)))
      (add `/Game/Blueprints/Stories/UI/BP_ActionBubble.OnLeftHandTrigger` _bubblereference_2 (delegate `Event OnLeftHandTriggered`))
      (add `/Game/Blueprints/Stories/UI/BP_ActionBubble.OnRightHandTrigger` _bubblereference_2 (delegate `Event OnRightHandTriggered`))
      (add `/Game/Blueprints/Stories/UI/BP_ActionBubble.OnAnyHandTrigger` _bubblereference_2 (delegate `Event OnAnyHandTriggered`)))))

(event `Event OnLeftHandTriggered`
  (`self.LeftHandTriggered`))

(event `Event OnRightHandTriggered`
  (`self.RightHandTriggered`))

(event `Event OnAnyHandTriggered`
  (`self.AnyHandTriggered`))

(fn `AnyHandTriggered`)

(fn `LeftHandTriggered`)

(fn `RightHandTriggered`)

(fn `SpawnBubble`
  (params (BubbleTransform :type "Transform Structure"))
  (returns (BubbleReference :type "/Game/Blueprints/Stories/UI/BP_ActionBubble Object Reference"))
  (bind _returnvalue (`|SpawnActorFromClass` "/Game/Blueprints/Stories/UI/BP_ActionBubble.BP_ActionBubble_C" BubbleTransform "Undefined" "MultiplyWithRoot" null null))
  (bind _output_get (set `self.BubbleComponent` _returnvalue))
  (return _output_get))

(fn `UserConstructionScript`
  (`parent.UserConstructionScript`))