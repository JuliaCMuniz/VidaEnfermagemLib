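; Base story teller that is meant to play an ordered list of stories in sequence.
; On BeginPlay it takes the first story and listens for its finished event, then unbinds and calls UpdateStory to pick and bind the next.
; UpdateStory signals the teller's end after the last entry.
; Its advance check compares list length as less than the next index, so as written it never moves to another story.
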(event `self.ReceiveBeginPlay`
  (if (> (`KismetArrayLibrary.Array_Length` (`self.StoryList`)) 0)
    (bind _output_get (set `self.CurrentStory` (`|GetArrayItem` (`self.StoryList`))))
    (add `/Game/Blueprints/Stories/BP_StoryBase.OnStoryFinished` (`|ConvertAsset` _output_get) (delegate `OnStoryFinished`))))

(event `OnStoryFinished`
  (remove `/Game/Blueprints/Stories/BP_StoryBase.OnStoryFinished` (`|ConvertAsset` (`self.CurrentStory`)) (delegate `OnStoryFinished`))
  (bind _storyresolved (`self.UpdateStory`))
  (add `/Game/Blueprints/Stories/BP_StoryBase.OnStoryFinished` _storyresolved (delegate `OnStoryFinished`)))

(fn `UpdateStory`
  (returns (StoryResolved :type "/Game/Blueprints/Stories/BP_StoryBase Object Reference"))
  (bind _storylist (`self.StoryList`))
  (bind _returnvalue (`KismetArrayLibrary.Array_Length` _storylist))
  (bind _returnvalue_2 (+ (`KismetArrayLibrary.Array_Find` _storylist (`self.CurrentStory`)) 1))
  (if (== _returnvalue _returnvalue_2)
    (`self.OnStoryTellerEnded`)
    (elif (< _returnvalue _returnvalue_2)
      (bind _output_get (set `self.CurrentStory` (`|GetArrayItem` (`self.StoryList`) _returnvalue_2)))
      (return (`|ConvertAsset` _output_get)))))

(fn `UserConstructionScript`)