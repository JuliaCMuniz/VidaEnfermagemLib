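; Dialogue component for the Mouse character, scripting a short branching conversation in which it asks for cheese.
; It overrides the parent Dialogue function and chains AddDialogue calls, branching on each returned state and option index.
; Saying No leads to a disappointed line, then clears progress and closes the conversation.
; Saying Yes offers give or keep choices, which have no follow-up wired.
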(fn `Dialogue`
  (`parent.Dialogue`)
  (switch `int` (`self.DialogueTreeIndex`)
    (:`Default`
      (bind (_state _optionindex) (`self.AddDialogue` "Mouse" "Hi, do you have any cheese?" (`|MakeArray` "Yes" "No" :!type "Text")))
      (switch `/Game/Blueprints/Interface/DialogueSystem/Enum_DialogueState` _state
        (:`NewEnumerator0`
          (switch `int` _optionindex
            (:`0`
              (bind (_state_2 _optionindex_2) (`self.AddDialogue` "Mouse" "Ahhh, that's great news! Can I have some?" (`|MakeArray` "Give Cheese" "Keep Cheese" :!type "Text")))
              (switch `/Game/Blueprints/Interface/DialogueSystem/Enum_DialogueState` _state_2
                (:`NewEnumerator0`
                  (switch `int` _optionindex_2))))
            (:`1`
              (bind _state_3 (`self.AddDialogue` "Mouse" "Awww, that's a shame! I really want some cheese." (`|MakeArray` "Continue" :!type "Text")))
              (switch `/Game/Blueprints/Interface/DialogueSystem/Enum_DialogueState` _state_3
                (:`NewEnumerator0`
                  (`self.ClearDialogueProgress`)
                  (`self.CloseConversation`))))))))))