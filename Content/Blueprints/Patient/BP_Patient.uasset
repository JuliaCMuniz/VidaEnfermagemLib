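; BP_Patient is a patient actor that glides from its spawn position toward a chair target.
; On BeginPlay it sets the target at a fixed X offset from its location and enables query and physics collision on the Remy component.
; Each Tick it eases toward that point with VInterpTo and a swept move until it is within one unit.
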(event `self.ReceiveBeginPlay`
  (set `self.TargetChair` (`KismetMathLibrary.MakeVector` (+ (.x (`self.K2_GetActorLocation` self)) 66.304166) (.y (`self.K2_GetActorLocation` self)) (.z (`self.K2_GetActorLocation` self))))
  (`PrimitiveComponent.SetCollisionEnabled` (`self.remy`) "QueryAndPhysics"))

(event `self.ReceiveTick`
  (params (DeltaSeconds :type "Float (single-precision)"))
  (bind _targetchair (`self.TargetChair`))
  (bind _returnvalue (`self.K2_GetActorLocation` self))
  (if (> (`KismetMathLibrary.Vector_Distance` _returnvalue _targetchair) 1.0)
    (`self.K2_SetActorLocation` self (`KismetMathLibrary.VInterpTo` _returnvalue _targetchair DeltaSeconds 0.6) true false)))

(fn `UserConstructionScript`)